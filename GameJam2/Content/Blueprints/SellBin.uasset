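; Sell bin actor that turns thrown fruit into gold for the player who owns it.
; An overlap with fruit-tagged actors advances that player's GlowIndicatorSystem once if it is at stage four, whether thrown or not.
; Thrown fruit adds its value to the owning Farmer's gold, is destroyed, and plays a sell sound.
; Tick re-runs this logic while the last overlapping actor remains inside, skipping the tag check.
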(event `self.Volume.OnComponentBeginOverlap`
  (params (OverlappedComponent :type "PrimitiveComponent Object Reference") (OtherActor :type "Actor Object Reference") (OtherComp :type "PrimitiveComponent Object Reference") (OtherBodyIndex :type Integer) (bFromSweep :type Boolean) (SweepResult :type "HitResult Structure (by ref)"))
  (if (`self.ActorHasTag` OtherActor "Fruit")
    (bind _asfruit_parent (cast `/Game/Blueprints/Fruits_Veggies/FruitParent` OtherActor :!label _label))
    (`|ExecutionSequence`
      (:`then_0`
        (bind _owningplayer (`/Game/Blueprints/Fruits_Veggies/FruitParent.OwningPlayer` _asfruit_parent))
        (if (== _owningplayer 0)
          (bind _returnvalue (`GameplayStatics.GetActorOfClass` "/Game/Blueprints/GlowIndicatorSystem.GlowIndicatorSystem_C"))
          (if (== (`/Game/Blueprints/GlowIndicatorSystem.Stages` _returnvalue) 4)
            (`/Engine/EditorBlueprintResources/StandardMacros.DoOnce` false
              (:`Completed`
                (`/Game/Blueprints/GlowIndicatorSystem.StageIncrease` _returnvalue))))
          (else
            (bind _returnvalue_2 (`GameplayStatics.GetActorOfClass` "/Game/Blueprints/GlowIndicatorSystem.GlowIndicatorSystem_C"))
            (if (== (`/Game/Blueprints/GlowIndicatorSystem.Stages2` _returnvalue_2) 4)
              (`/Engine/EditorBlueprintResources/StandardMacros.DoOnce` false
                (:`Completed`
                  (`/Game/Blueprints/GlowIndicatorSystem.Stage2Increase` _returnvalue_2)))))))
      (:`then_1`
        (if (`/Game/Blueprints/Fruits_Veggies/FruitParent.isThrown` _asfruit_parent)
          (bind _asfarmer (cast `/Game/Blueprints/Farmer` (`GameplayStatics.GetPlayerPawn` _owningplayer)))
          (set `/Game/Blueprints/Farmer.Gold` (+ (`/Game/Blueprints/Farmer.Gold` _asfarmer) (`/Game/Blueprints/Fruits_Veggies/FruitParent.value` _asfruit_parent)) _asfarmer)
          (`self.K2_DestroyActor` OtherActor)
          (`FMODBlueprintStatics.PlayEvent2D` "/Game/FMOD/Events/ShopAndUI/SellStuff.SellStuff"))))))

(event `self.ReceiveTick`
  (params (DeltaSeconds :type "Float (single-precision)"))
  (if (`self.IsOverlappingActor` (stale `self.Volume.OnComponentBeginOverlap` OtherActor))
    (goto _label)))

(fn `UserConstructionScript`)