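; Game instance that stores each player's fruit selection for up to four players.
; SaveFruitToSelection appends a fruit to the array matching the player index, with debug prints for the first player only.
; SelectDefaultFruits1 and 2 pad the first two players' selections to four with level actors found by class (Apple, Corn, Dragon, Pumpkin).
; Defaults follow array length, not contents, and the arrays hold actor references rather than classes.
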(fn `SaveFruitToSelection`
  (params (NewFruit :type "Actor Object Reference") (`Player Index` :type Integer))
  ;[1 1 1] Make sure to get player index for multiple players
  (switch `int` `Player Index`
    (:`0`
      (`KismetArrayLibrary.Array_Add` (`self.Player1Selection`) NewFruit)
      (`KismetSystemLibrary.PrintString` (`KismetSystemLibrary.GetDisplayName` NewFruit) true true (struct :`G` 0.66 :`B` 1.0 :`A` 1.0) 5.0)
      (`KismetSystemLibrary.PrintString` (`KismetSystemLibrary.GetClassDisplayName` (`GameplayStatics.GetObjectClass` NewFruit)) true true (struct :`G` 0.66 :`B` 1.0 :`A` 1.0) 5.0))
    (:`1`
      (`KismetArrayLibrary.Array_Add` (`self.Player2Selection`) NewFruit))
    (:`2`
      (`KismetArrayLibrary.Array_Add` (`self.Player3Selection`) NewFruit))
    (:`3`
      (`KismetArrayLibrary.Array_Add` (`self.Player4Selection`) NewFruit))))

(fn `SelectDefaultFruits1`
  (bind _player1selection (`self.Player1Selection`))
  (bind _returnvalue (`GameplayStatics.GetActorOfClass` (`self.Apple`)))
  (bind _returnvalue_2 (`GameplayStatics.GetActorOfClass` (`self.Corn`)))
  (bind _returnvalue_3 (`GameplayStatics.GetActorOfClass` (`self.Dragon`)))
  (bind _returnvalue_4 (`GameplayStatics.GetActorOfClass` (`self.Pumpkin`)))
  (switch `int` (`KismetArrayLibrary.Array_Length` _player1selection)
    (:`0`
      (`KismetArrayLibrary.Array_Add` _player1selection _returnvalue)
      (`KismetArrayLibrary.Array_Add` _player1selection _returnvalue_2)
      (`KismetArrayLibrary.Array_Add` _player1selection _returnvalue_3)
      (`KismetArrayLibrary.Array_Add` _player1selection _returnvalue_4))
    (:`1`
      (`KismetArrayLibrary.Array_Add` _player1selection _returnvalue_2)
      (`KismetArrayLibrary.Array_Add` _player1selection _returnvalue_3)
      (`KismetArrayLibrary.Array_Add` _player1selection _returnvalue_4))
    (:`2`
      (`KismetArrayLibrary.Array_Add` _player1selection _returnvalue_3)
      (`KismetArrayLibrary.Array_Add` _player1selection _returnvalue_4))
    (:`3`
      (`KismetArrayLibrary.Array_Add` _player1selection _returnvalue_4))))

(fn `SelectDefaultFruits2`
  (bind _player2selection (`self.Player2Selection`))
  (bind _returnvalue (`GameplayStatics.GetActorOfClass` (`self.Apple`)))
  (bind _returnvalue_2 (`GameplayStatics.GetActorOfClass` (`self.Corn`)))
  (bind _returnvalue_3 (`GameplayStatics.GetActorOfClass` (`self.Dragon`)))
  (bind _returnvalue_4 (`GameplayStatics.GetActorOfClass` (`self.Pumpkin`)))
  (switch `int` (`KismetArrayLibrary.Array_Length` _player2selection)
    (:`0`
      (`KismetArrayLibrary.Array_Add` _player2selection _returnvalue)
      (`KismetArrayLibrary.Array_Add` _player2selection _returnvalue_2)
      (`KismetArrayLibrary.Array_Add` _player2selection _returnvalue_3)
      (`KismetArrayLibrary.Array_Add` _player2selection _returnvalue_4))
    (:`1`
      (`KismetArrayLibrary.Array_Add` _player2selection _returnvalue_2)
      (`KismetArrayLibrary.Array_Add` _player2selection _returnvalue_3)
      (`KismetArrayLibrary.Array_Add` _player2selection _returnvalue_4))
    (:`2`
      (`KismetArrayLibrary.Array_Add` _player2selection _returnvalue_3)
      (`KismetArrayLibrary.Array_Add` _player2selection _returnvalue_4))
    (:`3`
      (`KismetArrayLibrary.Array_Add` _player2selection _returnvalue_4))))