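; Per-player loadout truck that collects fruit dropped onto it into its owner's selection, with a pink or blue decal by player.
; Overlapping same-owner fruit is destroyed and saved through MyGameInstance, unless its class matches the last entry in that player's selection, when it is only destroyed.
; After saving, the owner's Farmer releases carried fruit.
; Fruit overlaps also advance that player's GlowIndicatorLoadout once from stage three.
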(event `self.ReceiveBeginPlay`
  (bind _decal (`self.Decal`))
  (if (== (`self.OwningPlayerIndex`) 0)
    (`DecalComponent.SetDecalMaterial` _decal "/Game/Art/Textures/Glow/Decal_Pink.Decal_Pink")
    (else
      (`DecalComponent.SetDecalMaterial` _decal "/Game/Art/Textures/Glow/Decal_Blue.Decal_Blue"))))

(event `self.Collision.OnComponentBeginOverlap`
  (params (OverlappedComponent :type "PrimitiveComponent Object Reference") (OtherActor :type "Actor Object Reference") (OtherComp :type "PrimitiveComponent Object Reference") (OtherBodyIndex :type Integer) (bFromSweep :type Boolean) (SweepResult :type "HitResult Structure (by ref)"))
  (bind _owningplayerindex (`self.OwningPlayerIndex`))
  (if (`self.ActorHasTag` OtherActor "fruit")
    (bind _asfruit_parent (cast `/Game/Blueprints/Fruits_Veggies/FruitParent` OtherActor))
    (`|ExecutionSequence`
      (:`then_0`
        (if (== (`/Game/Blueprints/Fruits_Veggies/FruitParent.OwningPlayer` _asfruit_parent) _owningplayerindex)
          (if (== _owningplayerindex 0)
            (bind _asmy_game_instance (cast `/Game/Blueprints/MyGameInstance` (`GameplayStatics.GetGameInstance`)))
            (for _array_element (`/Game/Blueprints/MyGameInstance.Player1SelectionClasses` _asmy_game_instance)
              _)
            (if (== _array_element (`GameplayStatics.GetObjectClass` OtherActor))
              (`self.K2_DestroyActor` OtherActor)
              (else
                (set `self.CurrentFruit` _asfruit_parent :!label _label)
                (`self.K2_DestroyActor` _asfruit_parent)
                (`self.AddFruitToSelection`)
                (`KismetSystemLibrary.Delay` 0.2)
                (bind _outactors (`GameplayStatics.GetAllActorsOfClass` "/Game/Blueprints/Farmer.Farmer_C"))
                (for _array_element_2 _outactors
                  (if (== (`/Game/Blueprints/Farmer.PlayerNumber` _array_element_2) (`self.OwningPlayerIndex`))
                    (bind _children (`/Game/Blueprints/FBXImporter/FBXImporterUtils.GetAllAttachedActors` _array_element_2))
                    (if (not (== (`KismetArrayLibrary.Array_Length` _children) 0))
                      (`/Game/Blueprints/Farmer.RemoveFruit` _array_element_2))))))
            (else
              (bind _asmy_game_instance_2 (cast `/Game/Blueprints/MyGameInstance` (`GameplayStatics.GetGameInstance`)))
              (for _array_element_3 (`/Game/Blueprints/MyGameInstance.Player2SelectionClasses` _asmy_game_instance_2)
                _)
              (if (== _array_element_3 (`GameplayStatics.GetObjectClass` OtherActor))
                (`self.K2_DestroyActor` OtherActor)
                (else
                  (goto _label)))))))
      (:`then_1`
        (if (== _owningplayerindex 0)
          (bind _returnvalue (`GameplayStatics.GetActorOfClass` "/Game/Blueprints/GlowIndicatorLoadout.GlowIndicatorLoadout_C"))
          (if (== (`/Game/Blueprints/GlowIndicatorLoadout.Stages` _returnvalue) 3)
            (`/Engine/EditorBlueprintResources/StandardMacros.DoOnce` false
              (:`Completed`
                (`/Game/Blueprints/GlowIndicatorLoadout.StagesIncrease` _returnvalue))))
          (else
            (bind _returnvalue_2 (`GameplayStatics.GetActorOfClass` "/Game/Blueprints/GlowIndicatorLoadout.GlowIndicatorLoadout_C"))
            (if (== (`/Game/Blueprints/GlowIndicatorLoadout.Stages2` _returnvalue_2) 3)
              (`/Engine/EditorBlueprintResources/StandardMacros.DoOnce` false
                (:`Completed`
                  (`/Game/Blueprints/GlowIndicatorLoadout.Stages2Increase` _returnvalue_2))))))))))

(fn `AddFruitToSelection`
  (bind _asmy_game_instance (cast `/Game/Blueprints/MyGameInstance` (`GameplayStatics.GetGameInstance`))
    (:`then`
      (`/Game/Blueprints/MyGameInstance.SaveFruitToSelection` _asmy_game_instance (`self.CurrentFruit`) (`self.OwningPlayerIndex`)))
    (:`CastFailed`
      (`KismetSystemLibrary.PrintString` "cast failed"))))

(fn `UserConstructionScript`)