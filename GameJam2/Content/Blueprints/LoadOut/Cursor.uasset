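; Loadout cursor actor that lets a player hover over fruit buttons and add fruit types to a loadout list.
; It takes input from player 0, and the move axes offset it in the Y-Z plane.
; Capsule overlap with a FruitButton records the hovered fruit, which the pick-up/place action appends to the list and debug-prints.
; Per-player selection is only stubbed: the GameInstance cast leads nowhere and the Selection function is empty.
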(event `self.ReceiveBeginPlay`
  (`self.EnableInput` (`GameplayStatics.GetPlayerController` 0)))

(event `InputAction|PickUp/Place`
  (params (Key :type "Key Structure"))
  (bind _loadoutlist (`self.LoadoutList`))
  (:`Pressed`
    (`KismetArrayLibrary.Array_Add` (`self.LoadoutList`) (`self.Hovering`))
    (for (_ _array_index) _loadoutlist
      (`KismetSystemLibrary.PrintString` (`|GetEnumeratorNameAsString` (`|GetArrayItem` _loadoutlist _array_index))))))

(event `self.Capsule.OnComponentBeginOverlap`
  (params (OverlappedComponent :type "PrimitiveComponent Object Reference") (OtherActor :type "Actor Object Reference") (OtherComp :type "PrimitiveComponent Object Reference") (OtherBodyIndex :type Integer) (bFromSweep :type Boolean) (SweepResult :type "HitResult Structure (by ref)"))
  (bind _asfruit_button (cast `/Game/Blueprints/LoadOut/FruitButton` OtherActor))
  (set `self.Hovering` (`/Game/Blueprints/LoadOut/FruitButton.FruitType` _asfruit_button))
  ;[1 1 1] set up selection array for different players
  (cast `/Game/Blueprints/MyGameInstance` (`GameplayStatics.GetGameInstance`)))

(event `InputAxis|MoveForward`
  (params (AxisValue :type "Float (single-precision)"))
  (`self.K2_AddActorWorldOffset` (`KismetMathLibrary.MakeVector` 0.0 0.0 (* AxisValue 5.0))))

(event `InputAxis|MoveRight`
  (params (AxisValue :type "Float (single-precision)"))
  (`self.K2_AddActorWorldOffset` (`KismetMathLibrary.MakeVector` 0.0 (* AxisValue 5.0))))

(fn `Selection`)

(fn `UserConstructionScript`)