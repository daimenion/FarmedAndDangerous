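; DefaultApple is a loadout actor that supplies an apple as a player's default fruit selection.
; On BeginPlay it marks itself occupied, spawns a FruitApple just above its location and stores it as the current fruit.
; AddFruitToSelection then saves that fruit for the owning player index through MyGameInstance, printing an error if the cast fails.
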(event `self.ReceiveBeginPlay`
  (set `self.Occupied` true)
  (bind _returnvalue (`|SpawnActorFromClass` "/Game/Blueprints/Fruits_Veggies/FruitApple.FruitApple_C" (`KismetMathLibrary.MakeTransform` (+ (`self.K2_GetActorLocation`) (0.0 0.0 80.0))) "Undefined" "OverrideRootScale" null null))
  (set `self.CurrentFruit` _returnvalue)
  (`self.AddFruitToSelection`))

(fn `AddFruitToSelection`
  (bind _asmy_game_instance (cast `/Game/Blueprints/MyGameInstance` (`GameplayStatics.GetGameInstance`))
    (:`then`
      (`/Game/Blueprints/MyGameInstance.SaveFruitToSelection` _asmy_game_instance (`self.CurrentFruit`) (`self.Owning Player Index`)))
    (:`CastFailed`
      (`KismetSystemLibrary.PrintString` "cast failed"))))

(fn `UserConstructionScript`)