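; FruitParent is a fruit actor, named as a parent class, that can be held and thrown.
; ThrowStart swaps the held flag for thrown, but its Direction assignment is disconnected, so the passed NewDirection is never stored.
; While thrown, Tick moves it along normalized Direction by Speed and delta time, without sweep.
; Overlapping an actor tagged Player or Plant while thrown triggers Impact, which destroys the fruit.
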(event `self.ReceiveActorBeginOverlap`
  (params (OtherActor :type "Actor Object Reference"))
  (if (and (`self.isThrown`) (or (`self.ActorHasTag` OtherActor "Player") (`self.ActorHasTag` OtherActor "Plant")))
    (`self.impact`)))

(event `self.ReceiveTick`
  (params (DeltaSeconds :type "Float (single-precision)"))
  (if (`self.isThrown`)
    (`self.throw`)))

(fn `impact`
  (`self.K2_DestroyActor`))

(fn `throw`
  (`self.K2_SetActorTransform` (`KismetMathLibrary.MakeTransform` (+ (* (`KismetMathLibrary.Normal` (`self.direction`)) (* (`GameplayStatics.GetWorldDeltaSeconds`) (`self.speed`))) (.location (`SceneComponent.K2_GetComponentToWorld` (`self.DefaultSceneRoot`)))) (.rotation (`SceneComponent.K2_GetComponentToWorld` (`self.DefaultSceneRoot`))) (.scale (`SceneComponent.K2_GetComponentToWorld` (`self.DefaultSceneRoot`))))))

(fn `throwStart`
  (params (newDirection :type "Vector Structure"))
  (set `self.isThrown` true)
  (set `self.isHeld` false))

(fn `UserConstructionScript`)