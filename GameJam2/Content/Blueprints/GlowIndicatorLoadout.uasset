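; Two-player staged glow guide that highlights trees, then scarecrows, then trucks as each player progresses, and adds a GlowLoadOut widget on BeginPlay.
; Tick polls Farmers to advance a player's counter from stage 1 once they hold one item, hiding that player's tree highlights.
; StagesIncrease and Stages2Increase bump separate counters and run Stage2 and Stage3, which toggle per-player Scarecrow highlights and Truck decals through DoOnce gates.
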(event `self.ReceiveBeginPlay`
  (bind _outactors (`GameplayStatics.GetAllActorsOfClass` "/Game/Blueprints/Plants/TreeParents.TreeParents_C"))
  (for _array_element _outactors
    (`SceneComponent.SetHiddenInGame` (`/Game/Blueprints/Plants/TreeParents.Highlights` _array_element) false false))
  (bind _returnvalue (`|CreateWidget` "/Game/Blueprints/UI/GlowLoadOut.GlowLoadOut_C" (`GameplayStatics.GetPlayerController` 0)))
  (`UserWidget.AddToViewport` _returnvalue 0))

(event `self.ReceiveTick`
  (params (DeltaSeconds :type "Float (single-precision)"))
  (`|ExecutionSequence`
    (:`then_0`
      (if (!= (`self.Stages`) 1)
        (`/Engine/EditorBlueprintResources/StandardMacros.DoOnce` false
          (:`Completed`
            (bind _outactors (`GameplayStatics.GetAllActorsOfClass` "/Game/Blueprints/Plants/TreeParents.TreeParents_C"))
            (for _array_element _outactors
              (if (== (`/Game/Blueprints/Plants/TreeParents.OwningPlayer` _array_element) 0)
                (`SceneComponent.SetHiddenInGame` (`/Game/Blueprints/Plants/TreeParents.Highlights` _array_element) true false)))))))
    (:`then_1`
      (if (!= (`self.Stages2`) 1)
        (`/Engine/EditorBlueprintResources/StandardMacros.DoOnce` false
          (:`Completed`
            (bind _outactors_2 (`GameplayStatics.GetAllActorsOfClass` "/Game/Blueprints/Plants/TreeParents.TreeParents_C"))
            (for _array_element_2 _outactors_2
              (if (== (`/Game/Blueprints/Plants/TreeParents.OwningPlayer` _array_element_2) 1)
                (`SceneComponent.SetHiddenInGame` (`/Game/Blueprints/Plants/TreeParents.Highlights` _array_element_2) true false)))))))
    (:`then_2`
      (if (== (`self.Stages`) 1)
        (bind _outactors_3 (`GameplayStatics.GetAllActorsOfClass` "/Game/Blueprints/Farmer.Farmer_C"))
        (for _array_element_3 _outactors_3
          (if (== (`/Game/Blueprints/Farmer.HoldingNumberOfItems` _array_element_3) 1)
            (if (== (`/Game/Blueprints/Farmer.PlayerNumber` _array_element_3) 0)
              (`self.StagesIncrease`))))))
    (:`then_3`
      (if (== (`self.Stages2`) 1)
        (bind _outactors_4 (`GameplayStatics.GetAllActorsOfClass` "/Game/Blueprints/Farmer.Farmer_C"))
        (for _array_element_4 _outactors_4
          (if (== (`/Game/Blueprints/Farmer.HoldingNumberOfItems` _array_element_4) 1)
            (if (== (`/Game/Blueprints/Farmer.PlayerNumber` _array_element_4) 1)
              (`self.Stages2Increase`))))))))

(fn `Stage1`)

(fn `Stage2`
  (bind _stages (`self.Stages`))
  (bind _stages2 (`self.Stages2`))
  ;[1 1 1] Player1
  (`|ExecutionSequence`
    (:`then_0`
      (if (== _stages 2)
        (`/Engine/EditorBlueprintResources/StandardMacros.DoOnce` false
          (:`Completed`
            (bind _outactors (`GameplayStatics.GetAllActorsOfClass` "/Game/Blueprints/Scarecrow.Scarecrow_C"))
            (for _array_element _outactors
              (`SceneComponent.SetHiddenInGame` (`/Game/Blueprints/Scarecrow.Highlights` _array_element) false false))))
        (elif (> _stages 2)
          (`/Engine/EditorBlueprintResources/StandardMacros.DoOnce` false
            (:`Completed`
              (bind _outactors_2 (`GameplayStatics.GetAllActorsOfClass` "/Game/Blueprints/Scarecrow.Scarecrow_C"))
              (for _array_element_2 _outactors_2
                (`SceneComponent.SetHiddenInGame` (`/Game/Blueprints/Scarecrow.Highlights` _array_element_2) true false)))))))
    (:`then_1`
      ;[1 1 1] Player2
      (if (== _stages2 2)
        (`/Engine/EditorBlueprintResources/StandardMacros.DoOnce` false
          (:`Completed`
            (bind _outactors_3 (`GameplayStatics.GetAllActorsOfClass` "/Game/Blueprints/Scarecrow.Scarecrow_C"))
            (for _array_element_3 _outactors_3
              (`SceneComponent.SetHiddenInGame` (`/Game/Blueprints/Scarecrow.Highlights1` _array_element_3) false false))))
        (elif (> _stages2 2)
          (`/Engine/EditorBlueprintResources/StandardMacros.DoOnce` false
            (:`Completed`
              (bind _outactors_4 (`GameplayStatics.GetAllActorsOfClass` "/Game/Blueprints/Scarecrow.Scarecrow_C"))
              (for _array_element_4 _outactors_4
                (`SceneComponent.SetHiddenInGame` (`/Game/Blueprints/Scarecrow.Highlights1` _array_element_4) true false)))))))))

(fn `Stage3`
  (bind _stages (`self.Stages`))
  (bind _stages2 (`self.Stages2`))
  ;[1 1 1] Player1
  (`|ExecutionSequence`
    (:`then_0`
      (if (== _stages 3)
        (`/Engine/EditorBlueprintResources/StandardMacros.DoOnce` false
          (:`Completed`
            (bind _outactors (`GameplayStatics.GetAllActorsOfClass` "/Game/Blueprints/LoadOut/Truck.Truck_C"))
            (for _array_element _outactors
              (if (== (`/Game/Blueprints/LoadOut/Truck.OwningPlayerIndex` _array_element) 0)
                (`SceneComponent.SetHiddenInGame` (`/Game/Blueprints/LoadOut/Truck.Decal` _array_element) false false)))))
        (elif (> _stages 3)
          (`/Engine/EditorBlueprintResources/StandardMacros.DoOnce` false
            (:`Completed`
              (bind _outactors_2 (`GameplayStatics.GetAllActorsOfClass` "/Game/Blueprints/LoadOut/Truck.Truck_C"))
              (for _array_element_2 _outactors_2
                (if (== (`/Game/Blueprints/LoadOut/Truck.OwningPlayerIndex` _array_element_2) 0)
                  (`SceneComponent.SetHiddenInGame` (`/Game/Blueprints/LoadOut/Truck.Decal` _array_element_2) true false))))))))
    (:`then_1`
      ;[1 1 1] Player2
      (if (== _stages2 3)
        (`/Engine/EditorBlueprintResources/StandardMacros.DoOnce` false
          (:`Completed`
            (bind _outactors_3 (`GameplayStatics.GetAllActorsOfClass` "/Game/Blueprints/LoadOut/Truck.Truck_C"))
            (for _array_element_3 _outactors_3
              (if (== (`/Game/Blueprints/LoadOut/Truck.OwningPlayerIndex` _array_element_3) 1)
                (`SceneComponent.SetHiddenInGame` (`/Game/Blueprints/LoadOut/Truck.Decal` _array_element_3) false false)))))
        (elif (> _stages2 3)
          (`/Engine/EditorBlueprintResources/StandardMacros.DoOnce` false
            (:`Completed`
              (bind _outactors_4 (`GameplayStatics.GetAllActorsOfClass` "/Game/Blueprints/LoadOut/Truck.Truck_C"))
              (for _array_element_4 _outactors_4
                (if (== (`/Game/Blueprints/LoadOut/Truck.OwningPlayerIndex` _array_element_4) 1)
                  (`SceneComponent.SetHiddenInGame` (`/Game/Blueprints/LoadOut/Truck.Decal` _array_element_4) true false))))))))))

(fn `Stages2Increase`
  (`/Engine/EditorBlueprintResources/StandardMacros.IncrementInt` (`self.Stages2`)
    (:`  `
      (`self.Stage2`)
      (`self.Stage3`))))

(fn `StagesIncrease`
  (`/Engine/EditorBlueprintResources/StandardMacros.IncrementInt` (`self.Stages`)
    (:`  `
      (`self.Stage2`)
      (`self.Stage3`))))

(fn `UserConstructionScript`)