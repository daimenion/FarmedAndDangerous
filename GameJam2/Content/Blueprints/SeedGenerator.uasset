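; SeedGenerator is a destructible objective actor whose death triggers the win screen.
; On BeginPlay it passes MaxHealth to the Health widget in its widget component, then copies its current Health there every Tick.
; At zero or below, Tick adds a WinScreen to the viewport and destroys the actor after a short delay, with no guard against creating repeated screens during that delay.
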(event `self.ReceiveBeginPlay`
  (bind _ashealth (cast `/Game/Blueprints/UI/Health` (`WidgetComponent.GetUserWidgetObject` (`self.Widget`))))
  (set `/Game/Blueprints/UI/Health.MaxHealth` (`self.Max Health`) _ashealth))

(event `self.ReceiveTick`
  (params (DeltaSeconds :type "Float (single-precision)"))
  (bind _ashealth (cast `/Game/Blueprints/UI/Health` (`WidgetComponent.GetUserWidgetObject` (`self.Widget`))))
  (bind _output_get (set `/Game/Blueprints/UI/Health.CurrentHealth` (`self.Health`) _ashealth))
  (if (<= _output_get 0.0)
    (bind _returnvalue (`|CreateWidget` "/Game/Blueprints/UI/WinScreen.WinScreen_C"))
    (`UserWidget.AddToViewport` _returnvalue 0)
    (`KismetSystemLibrary.Delay` 0.1)
    (`self.K2_DestroyActor`)))

(fn `UserConstructionScript`)