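; Grid generator actor that spawns a square field of Grid actors, sized by GridSize, at runtime.
; BeginPlay seeds row and column counters; Tick builds one row per pass until rows run out.
; It acts as its own cursor, spawning at its transform, stepping along X, then rewinding and advancing along Y.
; A Delay ends each loop iteration, but a standard loop does not wait on it.
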(event `self.ReceiveBeginPlay`
  (bind _gridsize (`self.GridSize`))
  (set `self.Row` _gridsize)
  (set `self.Col` _gridsize))

(event `self.ReceiveTick`
  (params (DeltaSeconds :type "Float (single-precision)"))
  (bind _gridsize (`self.Gridsize`))
  (bind _col (`self.Col`))
  (bind _row (`self.Row`))
  (bind _returnvalue (`self.GetTransform` self))
  (bind _returnvalue_2 (`self.GetTransform` self))
  ;[1 1 1] GridSetup
  (if (> _row 0)
    (if (>= _col 0)
      (for _ (range 1 (+ _gridsize 1))
        (`|SpawnActorFromClass` "/Game/Blueprints/Grid/Grid.Grid_C" (`KismetMathLibrary.MakeTransform` (`KismetMathLibrary.MakeVector` (.x (.location _returnvalue)) (.y (.location _returnvalue)) (.z (.location _returnvalue))) (.rotation _returnvalue) (`KismetMathLibrary.MakeVector` (.x (.scale _returnvalue)) (.y (.scale _returnvalue)) (.z (.scale _returnvalue)))) "Undefined" "OverrideRootScale" null null)
        (set `self.Col` (- _col 1))
        (`self.K2_SetActorLocation` self (`KismetMathLibrary.MakeVector` (+ (.x (.location _returnvalue)) 200.0) (.y (.location _returnvalue)) (.z (.location _returnvalue))) false false)
        (`KismetSystemLibrary.Delay` 0.2))
      (`self.K2_SetActorLocation` self (`KismetMathLibrary.MakeVector` (- (.x (.location _returnvalue_2)) (* _gridsize 200.0)) (+ (.y (.location _returnvalue_2)) 200.0) (.z (.location _returnvalue_2))) false false)
      (set `self.Row` (- _row 1))
      (set `self.Col` _gridsize))))

(fn `UserConstructionScript`)