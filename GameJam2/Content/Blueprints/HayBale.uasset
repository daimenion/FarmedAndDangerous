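; HayBale is a destructible hay bale actor that loses health when hit by FruitCorn actors.
; On overlap with a FruitCorn, it subtracts CornDamage from HayHealth, reading the value from the first FruitCorn found in the world rather than the overlapping one.
; Tick checks HayHealth every frame and destroys the bale once it reaches zero or below.
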(event `self.ReceiveBeginPlay`
  (`parent.ReceiveBeginPlay`))

(event `self.ReceiveActorBeginOverlap`
  (params (OtherActor :type "Actor Object Reference"))
  (if (== (`GameplayStatics.GetObjectClass` OtherActor) "/Game/Blueprints/Fruits_Veggies/FruitCorn.FruitCorn_C")
    (bind _returnvalue (`GameplayStatics.GetActorOfClass` "/Game/Blueprints/Fruits_Veggies/FruitCorn.FruitCorn_C"))
    (bind _asfruit_corn (cast `/Game/Blueprints/Fruits_Veggies/FruitCorn` _returnvalue))
    (set `self.HayHealth` (- (`self.HayHealth`) (`/Game/Blueprints/Fruits_Veggies/FruitCorn.cornDamage` _asfruit_corn)))))

(event `self.ReceiveTick`
  (params (DeltaSeconds :type "Float (single-precision)"))
  (`parent.ReceiveTick` DeltaSeconds)
  (`|ExecutionSequence`
    (:`then_0`)
    (:`then_1`
      (`/Engine/EditorBlueprintResources/StandardMacros.CompareFloat` (`self.HayHealth`)
        (:`==`
          _)
        (:`<`
          _))
      (`self.K2_DestroyActor`))))

(fn `UserConstructionScript`
  (`parent.UserConstructionScript`))