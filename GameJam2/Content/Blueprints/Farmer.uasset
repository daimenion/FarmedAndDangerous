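; Playable farmer character for a two-player farming game, handling movement, pickup, planting, fruit throwing, selling and seed shopping.
; Overlap tags and the held-item count gate pickup and planting flags, while body-part meshes follow the main mesh's pose.
; The aim axes rotate an arrow and set the direction for respawning held fruit as a projectile.
; Overlapping a SellBin converts held fruit to gold, and a SeedGenerator opens that player's store widget.
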(event `self.ReceiveBeginPlay`
  (set `self.Gold` 10)
  (`SkinnedMeshComponent.SetLeaderPoseComponent` (`self.Hair`) (`self.Mesh`) false)
  (`SkinnedMeshComponent.SetLeaderPoseComponent` (`self.Belt`) (`self.Mesh`) false)
  (`SkinnedMeshComponent.SetLeaderPoseComponent` (`self.Face`) (`self.Mesh`) false)
  (`SkinnedMeshComponent.SetLeaderPoseComponent` (`self.Gloves`) (`self.Mesh`) false)
  (`SkinnedMeshComponent.SetLeaderPoseComponent` (`self.Shoes`) (`self.Mesh`) false)
  (`SkinnedMeshComponent.SetLeaderPoseComponent` (`self.HeadGear`) (`self.Mesh`) false))

(event `InputAxis|MoveForward`
  (params (AxisValue :type "Float (single-precision)"))
  (bind (_returnvalue_roll _returnvalue_pitch _returnvalue_yaw) (`KismetMathLibrary.BreakRotator` (`self.GetControlRotation`)))
  ;[1 1 1] Movement
  (`self.AddMovementInput` (`KismetMathLibrary.GetForwardVector` (`KismetMathLibrary.MakeRotator` 0.0 0.0 _returnvalue_yaw)) AxisValue))

(event `InputAction|PickUp/Place`
  (params (Key :type "Key Structure"))
  (:`Pressed`
    (`|ExecutionSequence`
      (:`then_0`
        (if (`self.NearTree`)
          (set `self.PickUpAFruit` true)))
      (:`then_1`
        (if (`self.NearSeed`)
          (set `self.PickUpSeed` true)))
      (:`then_2`
        (if (and (`self.PickUpSeed`) (== (`self.HoldingNumberOfItems`) 1))
          (set `self.PlantSeed` true)))))
  (:`Released`
    (`|ExecutionSequence`
      (:`then_0`
        (set `self.PickUpAFruit` false))
      (:`then_1`
        (set `self.PickUpSeed` false))
      (:`then_2`
        (set `self.PlantSeed` false)))))

(event `InputAxis|MoveRight`
  (params (AxisValue :type "Float (single-precision)"))
  (bind (_returnvalue_roll _returnvalue_pitch _returnvalue_yaw) (`KismetMathLibrary.BreakRotator` (`self.GetControlRotation`)))
  ;[1 1 1] Movement
  (`self.AddMovementInput` (`KismetMathLibrary.GetRightVector` (`KismetMathLibrary.MakeRotator` 0.0 0.0 _returnvalue_yaw)) AxisValue))

(event `self.ReceiveActorBeginOverlap`
  (params (OtherActor :type "Actor Object Reference"))
  (`|ExecutionSequence`
    (:`then_0`
      (if (`self.ActorHasTag` OtherActor "Trees")
        (set `self.NearTree` true)))
    (:`then_1`
      (if (`self.ActorHasTag` OtherActor "Seed")
        (set `self.NearSeed` true)))))

(event `InputAction|Throw`
  (params (Key :type "Key Structure"))
  (bind _returnvalue (`KismetMathLibrary.MakeVector` (`self.GetInputAxisValue`) (`self.GetInputAxisValue`)))
  (bind _output (`|GetArrayItem` (`self.GetAttachedActors`)))
  (bind _returnvalue_2 (`KismetMathLibrary.Conv_VectorToRotator` _returnvalue))
  ;[1 1 1] Throw
  (:`Pressed`
    (if (> (`self.HoldingNumberOfItems`) 0)
      (if (> (`KismetMathLibrary.VSize` _returnvalue) 0.0)
        (if (`self.ActorHasTag` _output "Fruit")
          (bind _returnvalue_3 (`|SpawnActorFromClass` (`GameplayStatics.GetObjectClass` _output) (`KismetMathLibrary.MakeTransform` (+ (`self.K2_GetActorLocation`) (`KismetMathLibrary.GreaterGreater_VectorRotator` (`self.FruitOffset`) _returnvalue_2)) _returnvalue_2) "AlwaysSpawn" "OverrideRootScale" null null))
          (`self.K2_DestroyActor` _output)
          (set `self.HoldingNumberOfItems` 0)
          (bind _asfruit_parent (cast `/Game/Blueprints/Fruits_Veggies/FruitParent` _returnvalue_3))
          (`ActorComponent.Activate` (`/Game/Blueprints/Fruits_Veggies/FruitParent.ProjectileMovement` _asfruit_parent) false)
          (set `/Game/Blueprints/Fruits_Veggies/FruitParent.isThrown` true _asfruit_parent))))))

(event `InputAxis|FireForward`
  (params (AxisValue :type "Float (single-precision)"))
  ;[1 1 1] Aiming Arrow
  (`SceneComponent.K2_SetWorldRotation` (`self.Arrow1`) (`KismetMathLibrary.Conv_VectorToRotator` (`KismetMathLibrary.MakeVector` AxisValue (stale `InputAxis|FireRight` AxisValue))) false false :!label _label))

(event `InputAction|OpenShops/Sell`
  (params (Key :type "Key Structure"))
  (bind _returnvalue (`GameplayStatics.GetPlayerController` 1))
  (bind _outactors (`self.GetAttachedActors`))
  (bind _returnvalue_2 (`GameplayStatics.GetPlayerController` 0))
  (:`Pressed`
    (`|ExecutionSequence`
      (:`then_0`
        (bind _outactors_2 (`GameplayStatics.GetAllActorsOfClass` "/Game/Blueprints/SellBin.SellBin_C"))
        (for _array_element _outactors_2
          (if (`self.IsOverlappingActor` _array_element self)
            (if (>= (`self.HoldingNumberOfItems`) 0)
              (bind _asfruit_parent (cast `/Game/Blueprints/Fruits_Veggies/FruitParent` (`|GetArrayItem` _outactors)))
              (set `self.Gold` (+ (`self.Gold`) (`/Game/Blueprints/Fruits_Veggies/FruitParent.value` _asfruit_parent)))
              (`self.K2_DestroyActor` _outactors)
              (set `self.HoldingNumberOfItems` 0)))))
      (:`then_1`
        (bind _outactors_3 (`GameplayStatics.GetAllActorsOfClass` "/Game/Blueprints/SeedGenerator.SeedGenerator_C"))
        (for _array_element_2 _outactors_3
          (if (`self.IsOverlappingActor` _array_element_2 self)
            (if (== (`self.PlayerNumber`) 0)
              (bind _returnvalue_3 (`|CreateWidget` "/Game/Blueprints/UI/Store01.Store01_C" _returnvalue_2))
              (`UserWidget.AddToViewport` _returnvalue_3 0)
              (`WidgetBlueprintLibrary.SetInputMode_UIOnlyEx` _returnvalue_2 _returnvalue_3)
              (`KismetSystemLibrary.Delay` 0.1)
              (`Widget.SetUserFocus` (`/Game/Blueprints/UI/Store01.Apple` _returnvalue_3) _returnvalue_2)
              (else
                (bind _returnvalue_4 (`|CreateWidget` "/Game/Blueprints/UI/Store02.Store02_C" _returnvalue))
                (`UserWidget.AddToViewport` _returnvalue_4 1)
                (`WidgetBlueprintLibrary.SetInputMode_UIOnlyEx` _returnvalue _returnvalue_4)
                (`KismetSystemLibrary.Delay` 0.1)
                (`Widget.SetUserFocus` (`/Game/Blueprints/UI/Store02.Apple` _returnvalue_4) _returnvalue)))))))))

(event `InputAxis|FireRight`
  (params (AxisValue :type "Float (single-precision)"))
  ;[1 1 1] Aiming Arrow
  (goto _label))

(event `self.ReceiveTick`
  (params (DeltaSeconds :type "Float (single-precision)"))
  (bind _arrow1 (`self.Arrow1`))
  ;[1 1 1] Aiming Arrow
  (if (> (`KismetMathLibrary.VSize` (`KismetMathLibrary.MakeVector` (stale `InputAxis|FireForward` AxisValue) (stale `InputAxis|FireRight` AxisValue))) 0.0)
    (`SceneComponent.SetHiddenInGame` _arrow1 false false)
    (else
      (`SceneComponent.SetHiddenInGame` _arrow1 true false))))

(fn `UserConstructionScript`)