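; Cart is an actor with a health bar widget that removes itself when its health runs out.
; On BeginPlay it casts the widget component's user widget to Health and sets the maximum health.
; Each Tick it repeats the cast, copies its own Health variable into the widget's CurrentHealth, and destroys the actor when that value reaches zero or below.
; Nothing in this file changes the Health variable.
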(event `self.ReceiveBeginPlay`
  (bind _ashealth (cast `/Game/Blueprints/UI/Health` (`WidgetComponent.GetUserWidgetObject` (`self.Widget`))))
  (set `/Game/Blueprints/UI/Health.MaxHealth` 10.0 _ashealth))

(event `self.ReceiveTick`
  (params (DeltaSeconds :type "Float (single-precision)"))
  (bind _ashealth (cast `/Game/Blueprints/UI/Health` (`WidgetComponent.GetUserWidgetObject` (`self.Widget`))))
  (bind _output_get (set `/Game/Blueprints/UI/Health.CurrentHealth` (`self.Health`) _ashealth))
  (if (<= _output_get 0.0)
    (`self.K2_DestroyActor`)))

(fn `UserConstructionScript`)