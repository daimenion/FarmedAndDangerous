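; Pomegranate fruit projectile, a child fruit class thrown without an arc as a single-shot clip, that bursts into shrapnel.
; BeginPlay sets its stats, seed and icon; once thrown, a delayed fuse calls Impact and destroys it unless it has already burst.
; Impact plays a splat, spawns shrapnel, flags it as spawned, then runs the parent impact.
; Shrapnel pieces get randomized offsets, roll and yaw, inherit the owning player and launch as thrown projectiles.
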(event `self.ReceiveBeginPlay`
  (`parent.ReceiveBeginPlay`)
  (set `self.IsArcThrowing` false)
  (set `self.speed` (`self.pomegSpeed`))
  (set `self.damage` (`self.pomegDamage`))
  (set `self.value` (`self.pomegValue`))
  (set `self.FruitSeed` "/Game/Blueprints/Plants/PomegranateSeed.PomegranateSeed_C")
  (set `self.ClipSize` 1)
  (set `self.ArcStrength` 0.0)
  (set `self.Icon` "/Game/Art/Textures/Pomegranate/Pomegranate_V2.Pomegranate_V2"))

(event `self.ReceiveActorBeginOverlap`
  (params (OtherActor :type "Actor Object Reference"))
  (`parent.ReceiveActorBeginOverlap` OtherActor))

(event `self.ReceiveTick`
  (params (DeltaSeconds :type "Float (single-precision)"))
  (if (`self.isThrown`)
    (`KismetSystemLibrary.Delay` (`self.delay`))
    (`/Engine/EditorBlueprintResources/StandardMacros.DoOnce` false
      (:`Completed`
        (if (not (`self.Spawned`))
          (`self.impact` null)
          (`self.K2_DestroyActor`))))))

(fn `impact`
  (params (other :type "Actor Object Reference"))
  (returns (ignoreMe :type Boolean))
  (`GameplayStatics.SpawnSoundAtLocation` "/Game/Audio/fruitSplat.fruitSplat" (`self.K2_GetActorLocation`) (struct) 1.0 1.0 0.0 null null)
  (`self.spawnShrapnel`)
  (set `self.Spawned` true)
  (bind _ignoreme (`parent.impact` other))
  (return _ignoreme))

(fn `spawnShrapnel`
  (bind (_returnvalue_roll _returnvalue_pitch _returnvalue_yaw) (`KismetMathLibrary.BreakRotator` (`self.K2_GetActorRotation`)))
  (bind _shrapnelrotation (`self.shrapnelRotation`))
  (`FMODBlueprintStatics.PlayEventAtLocation` "/Game/FMOD/Events/ThrownSound/PomScatter.PomScatter" (`self.GetTransform`))
  (for _ (range 1 (+ (`self.shrapnelAmount`) 1))
    (bind _returnvalue (`|SpawnActorFromClass` "/Game/Blueprints/Fruits_Veggies/FruitPomegranate_Shrapnel.FruitPomegranate_Shrapnel_C" (`KismetMathLibrary.MakeTransform` (+ (`self.K2_GetActorLocation`) (`KismetMathLibrary.MakeVector` (`KismetMathLibrary.RandomFloatInRange` 0.0 100.0) 0.0 (`KismetMathLibrary.RandomFloatInRange` 0.0 100.0))) (`KismetMathLibrary.MakeRotator` (`KismetMathLibrary.RandomFloatInRange` (- _returnvalue_roll 20.0) (+ _returnvalue_roll _shrapnelrotation)) 0.0 (`KismetMathLibrary.RandomFloatInRange` (- _returnvalue_yaw 20.0) (+ _returnvalue_yaw _shrapnelrotation)))) "Undefined" "OverrideRootScale" null null))
    (set `/Game/Blueprints/Fruits_Veggies/FruitParent.OwningPlayer` (`self.OwningPlayer`) _returnvalue)
    (`ActorComponent.Activate` (`/Game/Blueprints/Fruits_Veggies/FruitParent.ProjectileMovement1` _returnvalue) false)
    (set `/Game/Blueprints/Fruits_Veggies/FruitParent.isThrown` true _returnvalue)))

(fn `UserConstructionScript`
  (`parent.UserConstructionScript`))