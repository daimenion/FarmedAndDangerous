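; FruitCoconut is the coconut fruit child Blueprint, an arc-thrown projectile that sets its own damage, value, seed, icon and splat decals.
; While falling, overlapping the Farmer whose player number matches OwningPlayer stuns them; otherwise overlaps defer to the parent.
; Impact plays a sound event, halts movement, removes the fruit component and activates particles.
; Particle collisions spawn random fading decals, while activation times the splat decal reveal, particle shutdown and actor destruction.
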(event `self.ReceiveBeginPlay`
  (`parent.ReceiveBeginPlay`)
  (set `self.damage` 15.0)
  (set `self.value` (`self.CoconutValue`))
  (set `self.FruitSeed` "/Game/Blueprints/Plants/CoconutSeed.CoconutSeed_C")
  (set `self.IsArcThrowing` true)
  (set `self.ClipSize` 1)
  (set `self.ArcStrength` 1.0)
  (set `self.Icon` "/Game/Art/Textures/Coconut/Coconut_V2.Coconut_V2")
  (set `self.SplatDecals` (`self.CoconutSplatArray`)))

(event `self.ReceiveActorBeginOverlap`
  (params (OtherActor :type "Actor Object Reference"))
  (if (`self.Falling`)
    (bind _asfarmer (cast `/Game/Blueprints/Farmer` OtherActor))
    (if (== (`self.OwningPlayer`) (`/Game/Blueprints/Farmer.PlayerNumber` _asfarmer))
      (set `/Game/Blueprints/Farmer.Stun` true _asfarmer))
    (else
      (`parent.ReceiveActorBeginOverlap` OtherActor))))

(event `self.MasterParticle.OnParticleCollide`
  (params (EventName :type Name) (EmitterTime :type "Float (single-precision)") (ParticleTime :type Integer) (Location :type "Vector Structure") (Velocity :type "Vector Structure") (Direction :type "Vector Structure") (Normal :type "Vector Structure") (BoneName :type Name) (PhysMat :type "PhysicalMaterial Object Reference"))
  (bind _coconutsplatarray (`self.CoconutSplatArray`))
  (bind _returnvalue (`GameplayStatics.SpawnDecalAtLocation` (`|GetArrayItem` _coconutsplatarray (`KismetMathLibrary.RandomIntegerInRange` 0 (- (`KismetArrayLibrary.Array_Length` _coconutsplatarray) 1))) (32.0 32.0 32.0) Location (`KismetMathLibrary.Conv_VectorToRotator` Direction) 8.0))
  (`DecalComponent.SetFadeOut` _returnvalue 0.0 6.5 true))

(event `self.MasterParticle.OnComponentActivated`
  (params (Component :type "ActorComponent Object Reference") (bReset :type Boolean))
  (bind _coconutsplatarray (`self.CoconutSplatArray`))
  (bind _splatdecal (`self.SplatDecal`))
  (`KismetSystemLibrary.Delay` 0.7)
  (`DecalComponent.SetDecalMaterial` _splatdecal (`|GetArrayItem` _coconutsplatarray (`KismetMathLibrary.RandomIntegerInRange` 0 (- (`KismetArrayLibrary.Array_Length` _coconutsplatarray) 1))))
  (`SceneComponent.SetVisibility` _splatdecal true false)
  (`KismetSystemLibrary.Delay` 2.0)
  (`ActorComponent.Deactivate` (`self.MasterParticle`))
  (`KismetSystemLibrary.Delay` 7.0)
  (`self.K2_DestroyActor`))

(fn `impact`
  (params (other :type "Actor Object Reference"))
  (returns (ignoreMe :type Boolean))
  (bind _projectilemovement1 (`self.ProjectileMovement1`))
  (`FMODBlueprintStatics.PlayEventAtLocation` "/Game/FMOD/Events/ImpactSound/ApplePotatoCoconutImpact.ApplePotatoCoconutImpact" (`self.GetTransform`))
  (set `ProjectileMovementComponent.ProjectileGravityScale` 0.0 _projectilemovement1)
  (set `MovementComponent.Velocity` (0.0 0.0 0.0) _projectilemovement1)
  (`ActorComponent.K2_DestroyComponent` (`self.Fruits`))
  (`ActorComponent.Activate` (`self.MasterParticle`) false)
  (bind _ignoreme (`parent.impact` null))
  (return _ignoreme))

(fn `UserConstructionScript`
  (`parent.UserConstructionScript`))