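; Corn variant of the fruit projectile, a child Blueprint that sets its own speed, damage, value, seed, icon and clip size on BeginPlay.
; Zero arc strength is set, and ThrowMultiple moves the actor along the normalized Direction by corn speed scaled by delta time, without sweep.
; Impact plays a splat sound at the actor's location, then defers to the parent's impact handling.
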(event `self.ReceiveBeginPlay`
  (`parent.ReceiveBeginPlay`)
  (set `self.ClipSize` 8)
  (set `self.speed` (`self.cornSpeed`))
  (set `self.damage` (`self.cornDamage`))
  (set `self.value` (`self.cornValue`))
  (set `self.FruitSeed` "/Game/Blueprints/Plants/CornSeed.CornSeed_C")
  (set `self.ArcStrength` 0.0)
  (set `self.Icon` "/Game/Art/Textures/Corn/Corn_V1.Corn_V1"))

(event `self.ReceiveActorBeginOverlap`
  (params (OtherActor :type "Actor Object Reference"))
  (`parent.ReceiveActorBeginOverlap` OtherActor))

(event `self.ReceiveTick`
  (params (DeltaSeconds :type "Float (single-precision)"))
  (`parent.ReceiveTick` DeltaSeconds))

(fn `impact`
  (params (other :type "Actor Object Reference"))
  (returns (ignoreMe :type Boolean))
  (`GameplayStatics.SpawnSoundAtLocation` "/Game/Audio/fruitSplat.fruitSplat" (`self.K2_GetActorLocation`) (struct) 1.0 1.0 0.0 null null)
  (bind _ignoreme (`parent.impact` other))
  (return _ignoreme))

(fn `ThrowMultiple`
  (`self.K2_SetActorTransform` (`KismetMathLibrary.MakeTransform` (+ (* (`KismetMathLibrary.Normal` (`self.direction`)) (* (`GameplayStatics.GetWorldDeltaSeconds`) (`self.cornSpeed`))) (.location (`SceneComponent.K2_GetComponentToWorld` (`self.DefaultSceneRoot`)))) (.rotation (`SceneComponent.K2_GetComponentToWorld` (`self.DefaultSceneRoot`))) (.scale (`SceneComponent.K2_GetComponentToWorld` (`self.DefaultSceneRoot`))))))

(fn `UserConstructionScript`
  (`parent.UserConstructionScript`))