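; Pumpkin fruit Blueprint, a child fruit class that adds splash damage when it hits.
; BeginPlay sets its damage, value, seed, a clip size of one and non-arced throwing on the inherited variables.
; Impact spawns a PumpkinExplosion and damages trees and carts overlapping its Splash component, excluding the hit actor, with matching hurt sounds.
; It then plays a splat and hands the hit actor to the parent Impact.
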(event `self.ReceiveBeginPlay`
  (`parent.ReceiveBeginPlay`)
  (set `self.damage` (`self.pumpkinDamage`))
  (set `self.value` (`self.PumpkinValue`))
  (set `self.FruitSeed` "/Game/Blueprints/Plants/PumpkinSeed.PumpkinSeed_C")
  (set `self.IsArcThrowing` false)
  (set `self.ClipSize` 1)
  (set `self.ArcStrength` 0.0))

(event `self.ReceiveActorBeginOverlap`
  (params (OtherActor :type "Actor Object Reference"))
  (`parent.ReceiveActorBeginOverlap` OtherActor))

(event `self.ReceiveTick`
  (params (DeltaSeconds :type "Float (single-precision)"))
  (`parent.ReceiveTick` DeltaSeconds))

(fn `impact`
  (params (other :type "Actor Object Reference"))
  (returns (ignoreMe :type Boolean))
  (bind _returnvalue (`|SpawnActorFromClass` "/Game/Blueprints/Fruits_Veggies/pumpkinExplosion.pumpkinExplosion_C" (`self.GetTransform`) "Undefined" "OverrideRootScale" null null))
  (for _array_element (`PrimitiveComponent.GetOverlappingActors` (`/Game/Blueprints/Fruits_Veggies/pumpkinExplosion.Splash` _returnvalue) null)
    (if (!= _array_element other)
      (bind _astree_parents (cast `/Game/Blueprints/Plants/TreeParents` _array_element)
        (:`then`
          (set `/Game/Blueprints/Plants/TreeParents.Health` (- (`/Game/Blueprints/Plants/TreeParents.Health` _astree_parents) (`self.pumpkinSplashDamage`)) _astree_parents)
          (`GameplayStatics.SpawnSoundAtLocation` "/Game/Audio/plantHurt.plantHurt" (`self.K2_GetActorLocation` _astree_parents) (struct) 1.0 1.0 0.0 null null))
        (:`CastFailed`
          (bind _ascart (cast `/Game/Blueprints/Cart` _array_element))
          (set `/Game/Blueprints/Cart.Health` (- (`/Game/Blueprints/Cart.Health` _ascart) (`self.pumpkinSplashDamage`)) _ascart)
          (`GameplayStatics.SpawnSoundAtLocation` "/Game/Audio/woodBreak.woodBreak" (`self.K2_GetActorLocation` _ascart) (struct) 1.0 1.0 0.0 null null)))))
  (`GameplayStatics.SpawnSoundAtLocation` "/Game/Audio/pumpkinSplat.pumpkinSplat" (`self.K2_GetActorLocation`) (struct) 1.0 1.0 0.0 null null)
  (bind _ignoreme (`parent.impact` other))
  (return _ignoreme))

(fn `UserConstructionScript`
  (`parent.UserConstructionScript`))