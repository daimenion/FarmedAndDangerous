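; Watermelon fruit Blueprint, a child of a shared fruit class that acts as a throwable with its own damage, value and seed.
; On BeginPlay it overrides the inherited Damage, Value and FruitSeed with watermelon-specific values and turns on arc throwing.
; Its Impact override plays a watermelon splat sound at the actor's location, then returns the parent's impact result.
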(event `self.ReceiveBeginPlay`
  (`parent.ReceiveBeginPlay`)
  (set `self.damage` (`self.watermelonDamage`))
  (set `self.value` (`self.WatermelonValue`))
  (set `self.FruitSeed` "/Game/Blueprints/Plants/WatermelonSeed.WatermelonSeed_C")
  (set `self.IsArcThrowing` true))

(event `self.ReceiveActorBeginOverlap`
  (params (OtherActor :type "Actor Object Reference"))
  (`parent.ReceiveActorBeginOverlap` OtherActor))

(event `self.ReceiveTick`
  (params (DeltaSeconds :type "Float (single-precision)"))
  (`parent.ReceiveTick` DeltaSeconds))

(fn `impact`
  (params (other :type "Actor Object Reference"))
  (returns (ignoreMe :type Boolean))
  (`GameplayStatics.SpawnSoundAtLocation` "/Game/Audio/watermelonSplat.watermelonSplat" (`self.K2_GetActorLocation`) (struct) 1.0 1.0 0.0 null null)
  (bind _ignoreme (`parent.impact` other))
  (return _ignoreme))

(fn `UserConstructionScript`
  (`parent.UserConstructionScript`))