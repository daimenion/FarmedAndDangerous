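; FruitApple is the apple variant of a fruit actor, a child Blueprint that gives the apple its own speed, damage and value.
; On BeginPlay it runs the parent logic, then copies AppleSpeed, AppleDamage and AppleValue into the Speed, Damage and Value variables.
; Overlap, Tick and construction only forward to the parent, so all behavior beyond these stats comes from the parent class.
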(event `self.ReceiveBeginPlay`
  (`parent.ReceiveBeginPlay`)
  (set `self.speed` (`self.appleSpeed`))
  (set `self.damage` (`self.appleDamage`))
  (set `self.value` (`self.appleValue`)))

(event `self.ReceiveActorBeginOverlap`
  (params (OtherActor :type "Actor Object Reference"))
  (`parent.ReceiveActorBeginOverlap` OtherActor))

(event `self.ReceiveTick`
  (params (DeltaSeconds :type "Float (single-precision)"))
  (`parent.ReceiveTick` DeltaSeconds))

(fn `UserConstructionScript`
  (`parent.UserConstructionScript`))