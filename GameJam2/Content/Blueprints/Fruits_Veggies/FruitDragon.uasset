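; Dragon fruit variant of a throwable, arc-thrown fruit that sets trees not owned by the thrower on fire and scorches the ground.
; It sets its stats on BeginPlay and arms once its Y velocity passes a threshold.
; Impact with a tree stops the projectile and activates a fire particle.
; That activation starts a timeline driving flame size and a dynamic-material burn decal, then the actor is destroyed after a delay.
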(event `self.ReceiveBeginPlay`
  (`parent.ReceiveBeginPlay`)
  (set `self.damage` (`self.dragonDamage`))
  (set `self.value` (`self.dragonValue`))
  (set `self.FruitSeed` "/Game/Blueprints/Plants/DragonSeed.DragonSeed_C")
  (set `self.ClipSize` 1)
  (set `self.IsArcThrowing` true)
  (set `self.Icon` "/Game/Art/Textures/DragonFruit/Dragon_Fruit_V1.Dragon_Fruit_V1"))

(event `self.ReceiveActorBeginOverlap`
  (params (OtherActor :type "Actor Object Reference"))
  (if (`self.ActorHasTag` OtherActor "Trees")
    (if (`self.isThrown`)
      (bind _astree_parents (cast `/Game/Blueprints/Plants/TreeParents` OtherActor)
        (:`then`
          (if (`/Game/Blueprints/Plants/TreeParents.LoadOut` _astree_parents)
            _
            (elif (!= (`/Game/Blueprints/Plants/TreeParents.OwningPlayer` _astree_parents) (`self.OwningPlayer`))
              (set `/Game/Blueprints/Plants/TreeParents.OnFire` true _astree_parents))))
        (:`CastFailed`
          _))))
  (`parent.ReceiveActorBeginOverlap` OtherActor) ; Do the standard collision stuff here. Everything past is for scorching
)

(event `self.ReceiveTick`
  (params (DeltaSeconds :type "Float (single-precision)"))
  (bind (_returnvalue_x _returnvalue_y) (`KismetMathLibrary.BreakVector` (`self.GetVelocity`)))
  (`parent.ReceiveTick` DeltaSeconds)
  (`/Engine/EditorBlueprintResources/StandardMacros.CompareFloat` _returnvalue_y 1.0 ; If dragonfruit has been thrown
    (:`>`
      (set `self.Armed` true) ; If dragonfruit can damage grid actors
    )))

(event `self.MasterParticle.OnComponentActivated`
  (params (Component :type "ActorComponent Object Reference") (bReset :type Boolean))
  (bind _splatdecal (`self.SplatDecal`))
  ;[1 1 1] Once activated launches event to set decal visability to true set the material with Dynamic material so can change the values on the Decal Component material
  (`SceneComponent.SetHiddenInGame` _splatdecal false false)
  (`DecalComponent.SetDecalMaterial` _splatdecal (`self.DynamicMaterial`))
  ;[1 1 1] Timeline to set values
  (bind (_direction _groundburn _flamesize) (`Timeline|Timeline_0` :!via `PlayFromStart`)
    (:`Update`
      ;[1 1 1] Vector Parameter will set the size of flames of particle effect in timeline. Scalar Paramater sets the mask of the decal to grow, and shrink using the Dynamic Material set in Contruction Script
      (`FXSystemComponent.SetVectorParameter` (`self.MasterParticle`) "FlameSize" _flamesize)
      (`MaterialInstanceDynamic.SetScalarParameterValue` (`self.DynamicMaterial`) "GroundBurn" _groundburn))
    (:`Finished`
      ;[1 1 1] Once timeline is finished after 3 second delay will destroy actor
      (`KismetSystemLibrary.Delay` 3.0)
      (`self.K2_DestroyActor`))
    (:`Deactivate`
      ;[1 1 1] Event plays at particular time in timeline to deactivate the particle effect
      (`ActorComponent.Deactivate` (`self.MasterParticle`)))))

(fn `impact`
  (params (other :type "Actor Object Reference"))
  (returns (ignoreMe :type Boolean))
  (cast `/Game/Blueprints/Plants/TreeParents` other)
  (`FMODBlueprintStatics.PlayEventAtLocation` "/Game/FMOD/Events/ImpactSound/Fire.Fire" (`self.GetTransform`))
  (set `MovementComponent.Velocity` (0.0 0.0 0.0) (`self.ProjectileMovement1`))
  (`ActorComponent.K2_DestroyComponent` (`self.Fruits`))
  (`ActorComponent.Activate` (`self.MasterParticle`) false)
  (bind _ignoreme (`parent.impact` other))
  (return _ignoreme))

(fn `UserConstructionScript`
  (bind _returnvalue (`KismetMaterialLibrary.CreateDynamicMaterialInstance` "/Game/Art/AshtonsContent/Materials/Instanced/INT_BurnedGround.INT_BurnedGround" "DM_Burn"))
  (set `self.DynamicMaterial` _returnvalue))