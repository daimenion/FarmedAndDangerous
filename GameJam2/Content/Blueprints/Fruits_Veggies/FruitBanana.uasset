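; Banana fruit, a child of a fruit base class, that is arc-thrown and turns into a banana peel when it lands on the grid.
; BeginPlay sets its stats, seed type and single-item clip after the parent's setup.
; While thrown, overlapping a Grid-tagged actor spawns a peel with the same owning player and destroys the banana; other overlaps go to the parent.
; Impact plays the watermelon splat sound before running parent logic.
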(event `self.ReceiveBeginPlay`
  (`parent.ReceiveBeginPlay`)
  (set `self.damage` 0.5)
  (set `self.value` 2)
  (set `self.FruitSeed` "/Game/Blueprints/Plants/BananaSeed.BananaSeed_C")
  (set `self.IsArcThrowing` true)
  (set `self.ClipSize` 1)
  (set `self.ArcStrength` 0.0))

(event `self.ReceiveActorBeginOverlap`
  (params (OtherActor :type "Actor Object Reference"))
  (if (`self.isThrown`)
    (if (`self.ActorHasTag` OtherActor "Grid")
      (bind _returnvalue (`|SpawnActorFromClass` "/Game/Blueprints/Fruits_Veggies/BananaPeel.BananaPeel_C" (`self.GetTransform`) "Undefined" "OverrideRootScale" null null))
      (set `/Game/Blueprints/Fruits_Veggies/BananaPeel.OwningPlayer` (`self.OwningPlayer`) _returnvalue)
      (`self.K2_DestroyActor`)
      (else
        (`parent.ReceiveActorBeginOverlap` OtherActor)))))

(fn `impact`
  (params (other :type "Actor Object Reference"))
  (returns (ignoreMe :type Boolean))
  (`GameplayStatics.SpawnSoundAtLocation` "/Game/Audio/watermelonSplat.watermelonSplat" (`self.K2_GetActorLocation`) (struct) 1.0 1.0 0.0 null null)
  (bind _ignoreme (`parent.impact` other))
  (return _ignoreme))

(fn `UserConstructionScript`
  (`parent.UserConstructionScript`))