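; FruitParent is the base actor for thrown fruit projectiles that damage opposing players' trees, seed generators and carts.
; BeginPlay configures the projectile movement as either an arc or a fast, plane-constrained straight throw.
; Overlaps filter by tag and owner before calling Impact, which applies damage, resolves fruit-versus-fruit hits by damage and triggers particles.
; Player stun exists in Impact, but its overlap branch is disconnected, as is the splat decal logic.
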(event `self.MasterParticle.OnParticleCollide`
  (params (EventName :type Name) (EmitterTime :type "Float (single-precision)") (ParticleTime :type Integer) (Location :type "Vector Structure") (Velocity :type "Vector Structure") (Direction :type "Vector Structure") (Normal :type "Vector Structure") (BoneName :type Name) (PhysMat :type "PhysicalMaterial Object Reference"))
  ;[1 1 1] Particle Effects
)

(event `self.MasterParticle.OnComponentActivated`
  (params (Component :type "ActorComponent Object Reference") (bReset :type Boolean))
  ;[1 1 1] Particle Effects
)

(event `self.ReceiveActorBeginOverlap`
  (params (OtherActor :type "Actor Object Reference"))
  (bind _returnvalue (`self.ActorHasTag` OtherActor "Grid"))
  (bind _owningplayer (`self.OwningPlayer`))
  (bind _owningplayer_2 (`self.OwningPlayer`))
  (if (and (`self.isThrown`) (or (`self.ActorHasTag` OtherActor "Player") (`self.ActorHasTag` OtherActor "Trees") (`self.ActorHasTag` OtherActor "SeedGenerator") (`self.ActorHasTag` OtherActor "Cart") (`self.ActorHasTag` OtherActor "Fruit") _returnvalue (`self.ActorHasTag` OtherActor "Hay")))
    (`|ExecutionSequence`
      (:`then_0`
        (bind _astree_parents (cast `/Game/Blueprints/Plants/TreeParents` OtherActor))
        (if (not (== (`/Game/Blueprints/Plants/TreeParents.OwningPlayer` _astree_parents) _owningplayer_2))
          (`self.impact` OtherActor :!label _label)
          (`KismetSystemLibrary.Delay` (`self.DelayBeforeDestroy`))
          (`self.K2_DestroyActor`)))
      (:`then_1`
        (bind _asseed_generator (cast `/Game/Blueprints/SeedGenerator` OtherActor))
        (if (not (== (`/Game/Blueprints/SeedGenerator.OwningPlayer` _asseed_generator) _owningplayer_2))
          (goto _label)))
      (:`then_2`
        (bind _ascart (cast `/Game/Blueprints/Cart` OtherActor))
        (if (== (`/Game/Blueprints/Cart.OwningPlayer` _ascart) _owningplayer_2)
          (`self.K2_DestroyActor`)
          (else
            (goto _label))))
      (:`then_3`
        (bind _asfruit_parent (cast `/Game/Blueprints/Fruits_Veggies/FruitParent` OtherActor))
        (if (not (== (`/Game/Blueprints/Fruits_Veggies/FruitParent.OwningPlayer` _asfruit_parent) _owningplayer))
          (`KismetSystemLibrary.Delay` 0.2)
          (goto _label)))
      (:`then_4`
        (if _returnvalue
          (goto _label)))
      (:`then_5`
        (bind _ashay_bale_5_2 (cast `/Game/Blueprints/Plants/HayBale5_2` OtherActor))
        (if (not (== _owningplayer (`/Game/Blueprints/Plants/HayBale5_2.OwningPlayerHayBale` _ashay_bale_5_2)))
          (goto _label))))))

(event `self.ReceiveBeginPlay`
  (bind _projectilemovement1 (`self.ProjectileMovement1`))
  ;[1 1 1] Type of  Throw
  (`KismetSystemLibrary.Delay` 0.05)
  (if (`self.IsArcThrowing`)
    (`ProjectileMovementComponent.SetVelocityInLocalSpace` _projectilemovement1 (`KismetMathLibrary.MakeVector` (`self.ArcStrength`) 0.0 1.0))
    (else
      (`MovementComponent.SetPlaneConstraintEnabled` _projectilemovement1 true)
      (`MovementComponent.SetPlaneConstraintNormal` _projectilemovement1 (0.0 0.0 1.0))
      (`ProjectileMovementComponent.SetVelocityInLocalSpace` _projectilemovement1 (3000.0 0.0 0.0))
      (set `ProjectileMovementComponent.InitialSpeed` 3000.0 _projectilemovement1)
      (set `ProjectileMovementComponent.MaxSpeed` 3000.0 _projectilemovement1))))

(event `self.ReceiveTick`
  (params (DeltaSeconds :type "Float (single-precision)"))
  ;[1 1 1] Type of  Throw
  (if (`self.isThrown`)
    (`KismetSystemLibrary.Delay` 15.0)
    (`self.K2_DestroyActor`)))

(fn `impact`
  (params (other :type "Actor Object Reference"))
  (returns (ignoreMe :type Boolean))
  (bind _projectilemovement1 (`self.ProjectileMovement1`))
  (`|ExecutionSequence`
    (:`then_0`
      (if (`self.ActorHasTag` other "Trees")
        (bind _astree_parents (cast `/Game/Blueprints/Plants/TreeParents` other))
        (if (not (`/Game/Blueprints/Plants/TreeParents.LoadOut` _astree_parents))
          (bind _output_get (set `/Game/Blueprints/Plants/TreeParents.Health` (- (`/Game/Blueprints/Plants/TreeParents.Health` _astree_parents) (`self.damage`)) _astree_parents))
          (if (not (<= _output_get 0.0))
            (`FMODBlueprintStatics.PlayEventAtLocation` "/Game/FMOD/Events/ImpactSound/PlantImpact.PlantImpact" (`self.GetTransform` _astree_parents))))
        (`ActorComponent.K2_DestroyComponent` (`self.Fruits`) :!label _label)
        (set `MovementComponent.Velocity` (0.0 0.0 0.0) _projectilemovement1)
        (set `ProjectileMovementComponent.ProjectileGravityScale` 0.0 _projectilemovement1)
        (`ActorComponent.Activate` (`self.MasterParticle`) false)
        (return false)))
    (:`then_1`
      (if (`self.ActorHasTag` other "SeedGenerator")
        (bind _asseed_generator (cast `/Game/Blueprints/SeedGenerator` other))
        (set `/Game/Blueprints/SeedGenerator.Health` (- (`/Game/Blueprints/SeedGenerator.Health` _asseed_generator) (`self.damage`)) _asseed_generator)
        (goto _label)))
    (:`then_2`
      (if (`self.ActorHasTag` other "Cart")
        (bind _ascart (cast `/Game/Blueprints/Cart` other))
        (set `/Game/Blueprints/Cart.Health` (- (`/Game/Blueprints/Cart.Health` _ascart) (`self.damage`)) _ascart)
        (`GameplayStatics.SpawnSoundAtLocation` "/Game/Audio/woodBreak.woodBreak" (`self.K2_GetActorLocation` _ascart) (struct) 1.0 1.0 0.0 null null)
        (goto _label)))
    (:`then_3`
      (if (`self.ActorHasTag` other "Player")
        (bind _asfarmer (cast `/Game/Blueprints/Farmer` other))
        (set `/Game/Blueprints/Farmer.Stun` true _asfarmer)))
    (:`then_4`
      (if (`self.ActorHasTag` other "Fruit")
        (bind _asfruit_parent (cast `/Game/Blueprints/Fruits_Veggies/FruitParent` other))
        (if (!= (`/Game/Blueprints/Fruits_Veggies/FruitParent.OwningPlayer` _asfruit_parent) (`self.OwningPlayer`))
          (`/Engine/EditorBlueprintResources/StandardMacros.CompareFloat` (`self.damage`) (`/Game/Blueprints/Fruits_Veggies/FruitParent.damage` _asfruit_parent)
            (:`==`
              (goto _label))
            (:`<`
              (goto _label))))))))

(fn `throw`
  (`self.K2_SetActorTransform` (`KismetMathLibrary.MakeTransform` (+ (* (`KismetMathLibrary.Normal` (`self.direction`)) (* (`GameplayStatics.GetWorldDeltaSeconds`) (`self.speed`))) (.location (`SceneComponent.K2_GetComponentToWorld` (`self.DefaultSceneRoot`)))) (.rotation (`SceneComponent.K2_GetComponentToWorld` (`self.DefaultSceneRoot`))) (.scale (`SceneComponent.K2_GetComponentToWorld` (`self.DefaultSceneRoot`))))))

(fn `throwStart`
  (params (newDirection :type "Vector Structure"))
  (set `self.isThrown` true)
  (set `self.isHeld` false))

(fn `UserConstructionScript`)