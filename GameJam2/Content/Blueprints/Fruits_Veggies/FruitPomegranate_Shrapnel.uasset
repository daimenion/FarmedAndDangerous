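; Pomegranate shrapnel projectile, a child fruit Blueprint that appears to be a fragment of the pomegranate fruit.
; On BeginPlay it copies its shrapnel speed, damage and value into Speed, Damage and Value, and sets FruitSeed to the pomegranate.
; Impact plays a fruit splat sound at its location, then defers to the parent's impact logic.
; Overlap handling and construction pass straight through to the parent.
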(event `self.ReceiveBeginPlay`
  (set `self.speed` (`self.shrapSpeed`))
  (set `self.damage` (`self.shrapDamage`))
  (set `self.value` (`self.shrapValue`))
  (set `self.FruitSeed` "/Game/Blueprints/Fruits_Veggies/FruitPomegranate.FruitPomegranate_C"))

(event `self.ReceiveActorBeginOverlap`
  (params (OtherActor :type "Actor Object Reference"))
  (`parent.ReceiveActorBeginOverlap` OtherActor))

(fn `impact`
  (params (other :type "Actor Object Reference"))
  (returns (ignoreMe :type Boolean))
  (`GameplayStatics.SpawnSoundAtLocation` "/Game/Audio/fruitSplat.fruitSplat" (`self.K2_GetActorLocation`) (struct) 1.0 1.0 0.0 null null)
  (bind _ignoreme (`parent.impact` other))
  (return _ignoreme))

(fn `UserConstructionScript`
  (`parent.UserConstructionScript`))