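; Carrot fruit projectile that, once thrown, damages trees, seed generators and carts not owned by its thrower's player.
; BeginPlay sets carrot speed, damage and value on inherited fields, with a single-item clip, no arc and an apple seed.
; Overlap filters by tag and owner, then calls Impact, which plays a splat, subtracts health and plays a target-specific hit sound.
; Player-tagged actors pass the overlap check but have no damage branch.
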(event `self.ReceiveBeginPlay`
  (`parent.ReceiveBeginPlay`)
  (set `self.speed` (`self.carrotSpeed`))
  (set `self.damage` (`self.carrotDamage`))
  (set `self.value` (`self.carrotValue`))
  (set `self.FruitSeed` "/Game/Blueprints/Plants/AppleSeed.AppleSeed_C")
  (set `self.ClipSize` 1)
  (set `self.ArcStrength` 0.0))

(event `self.ReceiveActorBeginOverlap`
  (params (OtherActor :type "Actor Object Reference"))
  (bind _owningplayer (`self.OwningPlayer`))
  (if (and (`self.isThrown`) (or (`self.ActorHasTag` OtherActor "Player") (`self.ActorHasTag` OtherActor "Trees") (`self.ActorHasTag` OtherActor "SeedGenerator") (`self.ActorHasTag` OtherActor "Cart")))
    (`|ExecutionSequence`
      (:`then_0`
        (bind _astree_parents (cast `/Game/Blueprints/Plants/TreeParents` OtherActor))
        (if (not (== (`/Game/Blueprints/Plants/TreeParents.OwningPlayer` _astree_parents) _owningplayer))
          (`self.impact` OtherActor :!label _label)))
      (:`then_1`
        (bind _asseed_generator (cast `/Game/Blueprints/SeedGenerator` OtherActor))
        (if (not (== (`/Game/Blueprints/SeedGenerator.OwningPlayer` _asseed_generator) _owningplayer))
          (goto _label)))
      (:`then_2`
        (bind _ascart (cast `/Game/Blueprints/Cart` OtherActor))
        (if (not (== (`/Game/Blueprints/Cart.OwningPlayer` _ascart) _owningplayer))
          (goto _label))))))

(event `self.ReceiveTick`
  (params (DeltaSeconds :type "Float (single-precision)"))
  (`parent.ReceiveTick` DeltaSeconds))

(fn `impact`
  (params (other :type "Actor Object Reference"))
  (returns (ignoreMe :type Boolean))
  (`GameplayStatics.SpawnSoundAtLocation` "/Game/Audio/fruitSplat.fruitSplat" (`self.K2_GetActorLocation`) (struct) 1.0 1.0 0.0 null null)
  (`|ExecutionSequence`
    (:`then_0`
      (if (`self.ActorHasTag` other "Trees")
        (bind _astree_parents (cast `/Game/Blueprints/Plants/TreeParents` other))
        (bind _output_get (set `/Game/Blueprints/Plants/TreeParents.Health` (- (`/Game/Blueprints/Plants/TreeParents.Health` _astree_parents) (`self.damage`)) _astree_parents))
        (if (not (<= _output_get 0.0))
          (`GameplayStatics.SpawnSoundAtLocation` "/Game/Audio/plantHurt.plantHurt" (`self.K2_GetActorLocation` _astree_parents) (struct) 1.0 1.0 0.0 null null)
          (return false))))
    (:`then_1`
      (if (`self.ActorHasTag` other "SeedGenerator")
        (bind _asseed_generator (cast `/Game/Blueprints/SeedGenerator` other))
        (set `/Game/Blueprints/SeedGenerator.Health` (- (`/Game/Blueprints/SeedGenerator.Health` _asseed_generator) (`self.damage`)) _asseed_generator)
        (`GameplayStatics.SpawnSoundAtLocation` "/Game/Audio/Mechanical.Mechanical" (`self.K2_GetActorLocation` _asseed_generator) (struct) 1.0 1.0 0.0 null null)
        (return false)))
    (:`then_2`
      (if (`self.ActorHasTag` other "Cart")
        (bind _ascart (cast `/Game/Blueprints/Cart` other))
        (set `/Game/Blueprints/Cart.Health` (- (`/Game/Blueprints/Cart.Health` _ascart) (`self.damage`)) _ascart)
        (`GameplayStatics.SpawnSoundAtLocation` "/Game/Audio/woodBreak.woodBreak" (`self.K2_GetActorLocation` _ascart) (struct) 1.0 1.0 0.0 null null)
        (return false)))))

(fn `UserConstructionScript`
  (`parent.UserConstructionScript`))