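; Potato projectile Blueprint, a child of a shared throwable fruit/veggie parent class that supplies the core behavior.
; On BeginPlay it copies potato-specific stats, seed and icon into inherited variables, with a single-item clip and arc throwing enabled at zero strength.
; Impact plays a sound event shared with apple and coconut, then defers to the parent.
; Particle system activation triggers delayed deactivation of the master particle, then destroys the actor.
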(event `self.ReceiveBeginPlay`
  (`parent.ReceiveBeginPlay`)
  (set `self.speed` (`self.potatoSpeed`))
  (set `self.damage` (`self.potatoDamage`))
  (set `self.value` (`self.potatoValue`))
  (set `self.FruitSeed` "/Game/Blueprints/Plants/potatoSeed.PotatoSeed_C")
  (set `self.ClipSize` 1)
  (set `self.ArcStrength` 0.0)
  (set `self.IsArcThrowing` true)
  (set `self.Icon` "/Game/Art/Textures/Potato/Potato_V1.Potato_V1"))

(event `self.ParticleSystem.OnComponentActivated`
  (params (Component :type "ActorComponent Object Reference") (bReset :type Boolean))
  (`KismetSystemLibrary.Delay` 1.0)
  (`ActorComponent.Deactivate` (`self.MasterParticle`))
  (`KismetSystemLibrary.Delay` 1.0)
  (`self.K2_DestroyActor`))

(fn `impact`
  (params (other :type "Actor Object Reference"))
  (returns (ignoreMe :type Boolean))
  (`FMODBlueprintStatics.PlayEventAtLocation` "/Game/FMOD/Events/ImpactSound/ApplePotatoCoconutImpact.ApplePotatoCoconutImpact" (`self.GetTransform`))
  (bind _ignoreme (`parent.impact` other))
  (return _ignoreme))

(fn `UserConstructionScript`
  (`parent.UserConstructionScript`))