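; Hay bale actor that acts as a seed pickup, attaching itself to a nearby Farmer.
; Each Tick it scans all Farmers and, for those within 210 units with nothing attached, sets PlayerIsNear based on a 200-unit threshold.
; Begin and end overlap with a Player-tagged Farmer also toggle that flag.
; While set, Tick attaches the bale to the loop's last Farmer element and updates its NearSeed and held-item count.
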(event `self.ReceiveTick`
  (params (DeltaSeconds :type "Float (single-precision)"))
  (`|ExecutionSequence`
    (:`then_0`
      ;[1 1 1] Detect if farmer is within 200 units
      (bind _outactors (`GameplayStatics.GetAllActorsOfClass` "/Game/Blueprints/Farmer.Farmer_C"))
      (for _array_element _outactors
        (bind _children (`/DatasmithContent/Blueprints/FBXImporter/FBXImporterUtils.GetAllAttachedActors` _array_element))
        (if (and (< (`self.GetDistanceTo` _array_element) 210.0) (== (`KismetArrayLibrary.Array_Length` _children) 0))
          (`/Engine/EditorBlueprintResources/StandardMacros.CompareFloat` (`self.GetDistanceTo` _array_element) 200.0
            (:`>`
              (set `self.PlayerIsNear` false))
            (:`==`
              (set `self.PlayerIsNear` true :!label _label))
            (:`<`
              (goto _label))))))
    (:`then_2`
      ;[1 1 1] Pick up seed
      (if (`self.PlayerIsNear`)
        (set `/Game/Blueprints/Farmer.NearSeed` true _array_element)
        (`self.K2_AttachToActor` _array_element "None" "KeepRelative" "KeepRelative" "KeepRelative")
        (set `/Game/Blueprints/Farmer.HoldingNumberOfItems` 1 _array_element)))))

(event `self.ReceiveActorEndOverlap`
  (params (OtherActor :type "Actor Object Reference"))
  (if (`self.ActorHasTag` OtherActor "Player")
    (cast `/Game/Blueprints/Farmer` OtherActor)
    (set `self.PlayerIsNear` false)))

(event `self.ReceiveActorBeginOverlap`
  (params (OtherActor :type "Actor Object Reference"))
  (if (`self.ActorHasTag` OtherActor "Player")
    (cast `/Game/Blueprints/Farmer` OtherActor)
    (set `self.PlayerIsNear` true)))

(fn `UserConstructionScript`)