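; CarrotTree is a plant Blueprint that configures a parent plant class to grow carrots.
; On BeginPlay it calls the parent, then sets the fruit to FruitCarrot along with its maximum count, health and fruit time.
; Tick and the construction script only call the parent, so the file adds no growth or harvest logic of its own.
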(event `self.ReceiveBeginPlay`
  (`parent.ReceiveBeginPlay`)
  (set `self.Fruits` "/Game/Blueprints/Fruits_Veggies/FruitCarrot.FruitCarrot_C")
  (set `self.MaxFruit` 1)
  (set `self.Health` 10.0)
  (set `self.FruitTime` 5.0))

(event `self.ReceiveTick`
  (params (DeltaSeconds :type "Float (single-precision)"))
  (`parent.ReceiveTick` DeltaSeconds))

(fn `UserConstructionScript`
  (`parent.UserConstructionScript`))