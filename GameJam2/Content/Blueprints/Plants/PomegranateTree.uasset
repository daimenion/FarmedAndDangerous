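; Pomegranate tree plant Blueprint that configures a parent plant class with its own fruit, seed and stats.
; On BeginPlay it calls the parent, then sets the pomegranate fruit and seed, fruit cap, health and fruit timing.
; It adds no other logic: Tick and overlap events are disabled, and the construction script only calls the parent.
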(event `self.ReceiveBeginPlay`
  (`parent.ReceiveBeginPlay`)
  (set `self.Fruits` "/Game/Blueprints/Fruits_Veggies/FruitPomegranate.FruitPomegranate_C")
  (set `self.MaxFruit` 2)
  (set `self.Health` 30.0)
  (set `self.FruitTime` 9.0)
  (set `self.Seed` "/Game/Blueprints/Plants/PomegranateSeed.PomegranateSeed_C"))

(fn `UserConstructionScript`
  (`parent.UserConstructionScript`))