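; WatermelonSeed is a seed Blueprint that defines the watermelon variant of a plantable item.
; On BeginPlay it sets its plant and tree references, growth timings and price, then calls the parent BeginPlay.
; It acts as a data-only override in practice, with no other active logic of its own, leaving behavior to the parent class.
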(event `self.ReceiveBeginPlay`
  (set `self.plant` "/Game/Blueprints/Plants/Pl_plant_03_Blueprint.Pl_plant_03_Blueprint_C")
  (set `self.Tree` "/Game/Blueprints/Plants/WatermelonTree.WatermelonTree_C")
  (set `self.PlantTime` 1.0)
  (set `self.TreeTime` 4.0)
  (set `self.Price` 5)
  (`parent.ReceiveBeginPlay`))

(fn `UserConstructionScript`
  (`parent.UserConstructionScript`))