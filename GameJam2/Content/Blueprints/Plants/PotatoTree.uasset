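; PotatoTree is a plant Blueprint that configures a potato-producing variant through variables on its parent class.
; On BeginPlay it calls the parent, then sets the fruit type, seed, fruit cap, fruit timer and health.
; It adds no other active logic, so any growth and fruiting behavior is left to the parent, whose BeginPlay runs before these values are assigned.
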(event `self.ReceiveBeginPlay`
  (`parent.ReceiveBeginPlay`)
  (set `self.Fruits` "/Game/Blueprints/Fruits_Veggies/VeggiePotato.VeggiePotato_C")
  (set `self.MaxFruit` 3)
  (set `self.Health` 30.0)
  (set `self.FruitTime` 5.0)
  (set `self.Seed` "/Game/Blueprints/Plants/potatoSeed.PotatoSeed_C"))

(fn `UserConstructionScript`
  (`parent.UserConstructionScript`))