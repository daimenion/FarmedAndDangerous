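; Fertilizer is a placeable plant-type item that marks the grid cell it is planted on as fertilized.
; BeginPlay sets its buy and seed-sell prices before calling the parent.
; Once Planted, each Tick scans all Grid actors, sets Fertilized on any within one unit, then destroys the fertilizer after a one-second delay.
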(event `self.ReceiveBeginPlay`
  (set `self.Price` 5.0)
  (set `self.sellSeedPrice` 3.0)
  (`parent.ReceiveBeginPlay`))

(event `self.ReceiveTick`
  (params (DeltaSeconds :type "Float (single-precision)"))
  (`parent.ReceiveTick` DeltaSeconds)
  (if (`self.Planted`)
    (bind _outactors (`GameplayStatics.GetAllActorsOfClass` "/Game/Blueprints/Grid/Grid.Grid_C"))
    (for _array_element _outactors
      (if (< (`self.GetDistanceTo` _array_element) 1.0)
        (bind _asgrid (cast `/Game/Blueprints/Grid/Grid` _array_element))
        (set `/Game/Blueprints/Grid/Grid.Fertilized` true _asgrid)
        (`KismetSystemLibrary.Delay` 1.0)
        (`self.K2_DestroyActor`)))))

(fn `UserConstructionScript`
  (`parent.UserConstructionScript`))