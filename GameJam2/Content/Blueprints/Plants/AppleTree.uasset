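; AppleTree is a plant Blueprint for a fruit-bearing apple tree, built as a child of a parent class.
; On BeginPlay it sets inherited-style settings for fruit type, fruit limit, health, fruit timing and seed, then calls the parent BeginPlay.
; All behavior is left to the parent, as the construction script only calls its parent and the Tick and overlap events are disabled.
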(event `self.ReceiveBeginPlay`
  (set `self.Fruits` "/Game/Blueprints/Fruits_Veggies/FruitApple.FruitApple_C")
  (set `self.MaxFruit` 3)
  (set `self.Health` 50.0)
  (set `self.FruitTime` 7.0)
  (set `self.Seed` "/Game/Blueprints/Plants/AppleSeed.AppleSeed_C")
  (`parent.ReceiveBeginPlay`))

(fn `UserConstructionScript`
  (`parent.UserConstructionScript`))