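; Destructible hay bale that loses health to the other player's thrown produce and is destroyed at zero, with seed pickup and planting logic also on it.
; Overlaps loop over every instance of the hit class, applying damage via UpdateHayHealth; FindNearest filters nothing.
; Tick polls Farmers to carry and plant it on empty Grid cells, spawns a Tree owned by map side, and restores the seed when that tree is gone.
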(event `self.ReceiveActorBeginOverlap`
  (params (OtherActor :type "Actor Object Reference"))
  (if (`self.ActorHasTag` OtherActor "Player")
    (cast `/Game/Blueprints/Farmer` OtherActor) ; If so, toggle whether the player is near
    (set `self.PlayerIsNear` true)
    (elif (`self.ActorHasTag` OtherActor "Fruit")
      (`|ExecutionSequence`
        (:`then_0`
          ;[1 1 1] Finding what type the colliding fruit is and getting the appropriate response
          (if (== (`GameplayStatics.GetObjectClass` OtherActor) "/Game/Blueprints/Fruits_Veggies/FruitCorn.FruitCorn_C")
            (bind _outactors (`GameplayStatics.GetAllActorsOfClass` "/Game/Blueprints/Fruits_Veggies/FruitCorn.FruitCorn_C")) ; Get all Corn possible
            (for _array_element _outactors
              (`self.Find Nearest` _array_element)
              (if (`/Game/Blueprints/Fruits_Veggies/FruitParent.isThrown` _array_element)
                (if (!= (`/Game/Blueprints/Fruits_Veggies/FruitParent.OwningPlayer` _array_element) (`self.OwningPlayerHayBale`))
                  (`self.UpdateHayHealth` _array_element (`/Game/Blueprints/Fruits_Veggies/FruitCorn.cornDamage` _array_element))
                  (else
                    (`self.K2_DestroyActor` _array_element)))))))
        (:`then_1`
          (if (== (`GameplayStatics.GetObjectClass` OtherActor) "/Game/Blueprints/Fruits_Veggies/FruitDragon.FruitDragon_C")
            (bind _outactors_2 (`GameplayStatics.GetAllActorsOfClass` "/Game/Blueprints/Fruits_Veggies/FruitDragon.FruitDragon_C"))
            (for _array_element_2 _outactors_2
              (`self.Find Nearest` _array_element_2)
              (if (`/Game/Blueprints/Fruits_Veggies/FruitParent.isThrown` _array_element_2)
                (if (!= (`/Game/Blueprints/Fruits_Veggies/FruitParent.OwningPlayer` _array_element_2) (`self.OwningPlayerHayBale`))
                  (`self.UpdateHayHealth` _array_element_2 (`/Game/Blueprints/Fruits_Veggies/FruitDragon.dragonDamage` _array_element_2))
                  (else
                    (`self.K2_DestroyActor` _array_element_2)))))))
        (:`then_2`
          (if (== (`GameplayStatics.GetObjectClass` OtherActor) "/Game/Blueprints/Fruits_Veggies/FruitApple.FruitApple_C")
            (bind _outactors_3 (`GameplayStatics.GetAllActorsOfClass` "/Game/Blueprints/Fruits_Veggies/FruitApple.FruitApple_C"))
            (for _array_element_3 _outactors_3
              (`self.Find Nearest` _array_element_3)
              (if (`/Game/Blueprints/Fruits_Veggies/FruitParent.isThrown` _array_element_3)
                (if (!= (`/Game/Blueprints/Fruits_Veggies/FruitParent.OwningPlayer` _array_element_3) (`self.OwningPlayerHayBale`))
                  (`self.UpdateHayHealth` _array_element_3 (`/Game/Blueprints/Fruits_Veggies/FruitApple.appleDamage` _array_element_3))
                  (else
                    (`self.K2_DestroyActor` _array_element_3)))))))
        (:`then_3`
          (if (== (`GameplayStatics.GetObjectClass` OtherActor) "/Game/Blueprints/Fruits_Veggies/FruitWatermelon.FruitWatermelon_C")
            (bind _outactors_4 (`GameplayStatics.GetAllActorsOfClass` "/Game/Blueprints/Fruits_Veggies/FruitWatermelon.FruitWatermelon_C"))
            (for _array_element_4 _outactors_4
              (`self.Find Nearest` _array_element_4)
              (if (`/Game/Blueprints/Fruits_Veggies/FruitParent.isThrown` _array_element_4)
                (if (!= (`/Game/Blueprints/Fruits_Veggies/FruitParent.OwningPlayer` _array_element_4) (`self.OwningPlayerHayBale`))
                  (`self.UpdateHayHealth` _array_element_4 (`/Game/Blueprints/Fruits_Veggies/FruitWatermelon.watermelonDamage` _array_element_4))
                  (else
                    (`self.K2_DestroyActor` _array_element_4)))))))
        (:`then_4`
          (if (== (`GameplayStatics.GetObjectClass` OtherActor) "/Game/Blueprints/Fruits_Veggies/FruitPomegranate.FruitPomegranate_C")
            (bind _outactors_5 (`GameplayStatics.GetAllActorsOfClass` "/Game/Blueprints/Fruits_Veggies/FruitPomegranate.FruitPomegranate_C"))
            (for _array_element_5 _outactors_5
              (`self.Find Nearest` _array_element_5)
              (if (`/Game/Blueprints/Fruits_Veggies/FruitParent.isThrown` _array_element_5)
                (if (!= (`/Game/Blueprints/Fruits_Veggies/FruitParent.OwningPlayer` _array_element_5) (`self.OwningPlayerHayBale`))
                  (`self.UpdateHayHealth` _array_element_5 (`/Game/Blueprints/Fruits_Veggies/FruitPomegranate.pomegDamage` _array_element_5))
                  (else
                    (`self.K2_DestroyActor` _array_element_5)))))))
        (:`then_5`
          (if (== (`GameplayStatics.GetObjectClass` OtherActor) "/Game/Blueprints/Fruits_Veggies/FruitPomegranate_Shrapnel.FruitPomegranate_Shrapnel_C")
            (bind _outactors_6 (`GameplayStatics.GetAllActorsOfClass` "/Game/Blueprints/Fruits_Veggies/FruitPomegranate_Shrapnel.FruitPomegranate_Shrapnel_C"))
            (for _array_element_6 _outactors_6
              (`self.Find Nearest` _array_element_6) ; Throw check is skipped because shrap only ever spawns after being thrown
              (if (!= (`/Game/Blueprints/Fruits_Veggies/FruitParent.OwningPlayer` _array_element_6) (`self.OwningPlayerHayBale`))
                (`self.UpdateHayHealth` _array_element_6 (`/Game/Blueprints/Fruits_Veggies/FruitPomegranate_Shrapnel.shrapDamage` _array_element_6))
                (else
                  (`self.K2_DestroyActor` _array_element_6))))))
        (:`then_6`
          (if (== (`GameplayStatics.GetObjectClass` OtherActor) "/Game/Blueprints/Fruits_Veggies/FruitCarrot.FruitCarrot_C")
            (bind _outactors_7 (`GameplayStatics.GetAllActorsOfClass` "/Game/Blueprints/Fruits_Veggies/FruitCarrot.FruitCarrot_C"))
            (for _array_element_7 _outactors_7
              (`self.Find Nearest` null)
              (if (`/Game/Blueprints/Fruits_Veggies/FruitParent.isThrown` _array_element_7)
                (if (!= (`/Game/Blueprints/Fruits_Veggies/FruitParent.OwningPlayer` _array_element_7) (`self.OwningPlayerHayBale`))
                  (`self.UpdateHayHealth` null (`/Game/Blueprints/Fruits_Veggies/FruitCarrot.carrotDamage` _array_element_7)) ; Do not destroy carrot
                )))))
        (:`then_7`
          (if (== (`GameplayStatics.GetObjectClass` OtherActor) "/Game/Blueprints/Fruits_Veggies/FruitPumpkin.FruitPumpkin_C")
            (bind _outactors_8 (`GameplayStatics.GetAllActorsOfClass` "/Game/Blueprints/Fruits_Veggies/FruitPumpkin.FruitPumpkin_C"))
            (for _array_element_8 _outactors_8
              (`self.Find Nearest` _array_element_8)
              (if (`/Game/Blueprints/Fruits_Veggies/FruitParent.isThrown` _array_element_8)
                (if (!= (`/Game/Blueprints/Fruits_Veggies/FruitParent.OwningPlayer` _array_element_8) (`self.OwningPlayerHayBale`))
                  (`self.UpdateHayHealth` _array_element_8 (`/Game/Blueprints/Fruits_Veggies/FruitPumpkin.pumpkinDamage` _array_element_8))
                  (else
                    (`self.K2_DestroyActor` _array_element_8)))))))
        (:`then_8`
          (if (== (`GameplayStatics.GetObjectClass` OtherActor) "/Game/Blueprints/Fruits_Veggies/VeggiePotato.VeggiePotato_C")
            (bind _outactors_9 (`GameplayStatics.GetAllActorsOfClass` "/Game/Blueprints/Fruits_Veggies/VeggiePotato.VeggiePotato_C"))
            (for _array_element_9 _outactors_9
              (`self.Find Nearest` _array_element_9)
              (if (`/Game/Blueprints/Fruits_Veggies/FruitParent.isThrown` _array_element_9)
                (if (!= (`/Game/Blueprints/Fruits_Veggies/FruitParent.OwningPlayer` _array_element_9) (`self.OwningPlayerHayBale`))
                  (`self.UpdateHayHealth` _array_element_9 (`/Game/Blueprints/Fruits_Veggies/VeggiePotato.potatoDamage` _array_element_9))
                  (else
                    (`self.K2_DestroyActor` _array_element_9)))))))
        (:`then_9`
          (if (== (`GameplayStatics.GetObjectClass` OtherActor) "/Game/Blueprints/Fruits_Veggies/FruitCoconut.FruitCoconut_C")
            (bind _outactors_10 (`GameplayStatics.GetAllActorsOfClass` "/Game/Blueprints/Fruits_Veggies/FruitCoconut.FruitCoconut_C"))
            (for _array_element_10 _outactors_10
              (`self.Find Nearest` _array_element_10)
              (if (`/Game/Blueprints/Fruits_Veggies/FruitParent.isThrown` _array_element_10)
                (`self.K2_DestroyActor` _array_element_10) ; Coconut does no damage
              ))))
        (:`then_10`
          (if (== (`GameplayStatics.GetObjectClass` OtherActor) "/Game/Blueprints/Fruits_Veggies/FruitBanana.FruitBanana_C")
            (bind _outactors_11 (`GameplayStatics.GetAllActorsOfClass` "/Game/Blueprints/Fruits_Veggies/FruitBanana.FruitBanana_C"))
            (for _array_element_11 _outactors_11
              (`self.Find Nearest` _array_element_11)
              (if (`/Game/Blueprints/Fruits_Veggies/FruitParent.isThrown` _array_element_11)
                (`self.K2_DestroyActor` _array_element_11) ; Banana does no damage
              ))))))))

(event `self.ReceiveBeginPlay`
  (set `self.Health` 10.0))

(event `self.ReceiveActorEndOverlap`
  (params (OtherActor :type "Actor Object Reference"))
  (if (`self.ActorHasTag` OtherActor "Player")
    (cast `/Game/Blueprints/Farmer` OtherActor)
    (set `self.PlayerIsNear` false)))

(event `self.ReceiveTick`
  (params (DeltaSeconds :type "Float (single-precision)"))
  (bind (_returnvalue_x _returnvalue_y _returnvalue_z) (`KismetMathLibrary.BreakVector` (`self.K2_GetActorLocation`)))
  ;[1 1 1] Seed
  (`|ExecutionSequence`
    (:`then_0`
      (if (`self.Planted`)
        (if (`self.IsSeed`)
          (set `self.IsSeed` false)
          (bind _returnvalue (`|SpawnActorFromClass` (`self.Tree`) (`self.GetTransform` self) "Undefined" "OverrideRootScale" null null))
          (set `self.IsTree` true)
          (bind (_returnvalue_x_2 _returnvalue_y_2) (`KismetMathLibrary.BreakVector` (`self.K2_GetActorLocation` _returnvalue)))
          (if (> _returnvalue_y_2 0.0)
            (bind _astree_parents (cast `/Game/Blueprints/Plants/TreeParents` _returnvalue))
            (set `/Game/Blueprints/Plants/TreeParents.OwningPlayer` 1 _astree_parents)
            (else
              (bind _astree_parents_2 (cast `/Game/Blueprints/Plants/TreeParents` _returnvalue))
              (set `/Game/Blueprints/Plants/TreeParents.OwningPlayer` 0 _astree_parents_2)))
          (set `self.myTree` _returnvalue))))
    (:`then_1`
      ;[1 1 1] Pick up seed
      (if (not (`self.destroyed`))
        (bind _outactors (`GameplayStatics.GetAllActorsOfClass` "/Game/Blueprints/Farmer.Farmer_C"))
        (for _array_element _outactors
          (bind _asfarmer (cast `/Game/Blueprints/Farmer` _array_element))
          (if (`self.IsOverlappingActor` _asfarmer self)
            (if (== (`/Game/Blueprints/Farmer.HoldingNumberOfItems` _asfarmer) 0)
              (if (`self.Planted`)
                _
                (elif (`/Game/Blueprints/Farmer.PickUpSeed` _asfarmer)
                  (`self.K2_SetActorLocation` (200.0 0.0 -20.0))
                  (`self.K2_AttachToActor` _asfarmer "None" "KeepRelative" "KeepRelative" "KeepRelative")
                  (set `/Game/Blueprints/Farmer.HoldingNumberOfItems` 1 _asfarmer))))))))
    (:`then_2`
      ;[1 1 1] Plant Seed
      (if (not (and (`self.Planted`) (`self.destroyed`)))
        (bind _outactors_2 (`GameplayStatics.GetAllActorsOfClass` "/Game/Blueprints/Farmer.Farmer_C"))
        (for _array_element_2 _outactors_2
          (bind _asfarmer_2 (cast `/Game/Blueprints/Farmer` _array_element_2))
          (if (`self.IsOverlappingActor` _array_element_2 self)
            (if (`/Game/Blueprints/Farmer.PickUpSeed` _asfarmer_2)
              (if (`/Game/Blueprints/Farmer.PlantSeed` _asfarmer_2)
                (bind _outactors_3 (`GameplayStatics.GetAllActorsOfClass` "/Game/Blueprints/Grid/Grid.Grid_C"))
                (for _array_element_3 _outactors_3
                  (bind _children (`/DatasmithContent/Blueprints/FBXImporter/FBXImporterUtils.GetAllAttachedActors` _array_element_3))
                  (if (and (< (`self.GetDistanceTo` _array_element_3) 200.0) (== (`KismetArrayLibrary.Array_Length` _children) 0))
                    (if (`self.IsSeed`)
                      (`self.K2_DetachFromActor` "KeepRelative")
                      (`self.K2_SetActorLocation` (`self.K2_GetActorLocation` _array_element_3))
                      (`self.K2_SetActorRotation` (struct :`Yaw` 90.0))
                      (`self.K2_AttachToActor` _array_element_3 "None" "KeepWorld" "KeepRelative" "KeepWorld")
                      (set `/Game/Blueprints/Farmer.HoldingNumberOfItems` 0 _asfarmer_2)
                      (set `self.Planted` true)
                      (`PrimitiveComponent.SetCollisionEnabled` (`self.Player Collider`) "NoCollision")
                      (`PrimitiveComponent.SetCollisionEnabled` (`self.Seed`) "NoCollision"))))))))))
    (:`then_3`
      ;[1 1 1] Destory seed
      (if (`self.IsTree`)
        (`GameplayStatics.GetActorOfClass` (`self.Tree`))
        (`/Engine/EditorBlueprintResources/StandardMacros.IsValid` _returnvalue
          (:`Is Not Valid`
            (`self.K2_DetachFromActor` "KeepWorld" "KeepWorld" "KeepWorld")
            (`self.K2_SetActorLocation` (`KismetMathLibrary.MakeVector` (- _returnvalue_x 200.0) _returnvalue_y _returnvalue_z))
            (`SceneComponent.SetHiddenInGame` (`self.Seed`) false false)
            (`PrimitiveComponent.SetCollisionEnabled` (`self.Player Collider`) "QueryAndPhysics")
            (`PrimitiveComponent.SetCollisionEnabled` (`self.Seed`) "QueryAndPhysics")
            (set `self.IsTree` false)
            (set `self.Planted` false)
            (set `self.IsSeed` true)
            (set `self.destroyed` true)))))
    (:`then_4`
      (if (`self.destroyed`)
        (bind _outactors_4 (`GameplayStatics.GetAllActorsOfClass` "/Game/Blueprints/Farmer.Farmer_C"))
        (for _array_element_4 _outactors_4
          (bind _asfarmer_3 (cast `/Game/Blueprints/Farmer` _array_element_4))
          (if (`self.IsOverlappingActor` _array_element_4 self)
            (if (== (`/Game/Blueprints/Farmer.HoldingNumberOfItems` _asfarmer_3) 0)
              (`KismetSystemLibrary.Delay` 0.2)
              (set `self.destroyed` false))))))
    (:`then_5`
      (`/Engine/EditorBlueprintResources/StandardMacros.CompareFloat` (`self.Health`)
        (:`==`
          _)
        (:`<`
          _))
      (`self.K2_DestroyActor`))))

(fn `Find Nearest`
  (params (`Actor To Test Dist On` :type "Actor Object Reference"))
  (`/DatasmithContent/Blueprints/FBXImporter/FBXImporterUtils.GetAllAttachedActors` null)
  (if (< (`self.GetDistanceTo` `Actor To Test Dist On`) 200.0)
    _))

(fn `UpdateHayHealth`
  (params (`Actor to Destroy On Impact` :type "Actor Object Reference") (`Reduce Health By` :type "Float (double-precision)"))
  (bind _output_get (set `self.Health` (- (`self.Health`) `Reduce Health By`))) ; Remove health from object
  (`self.K2_DestroyActor` `Actor to Destroy On Impact`) ; Destroy corn
  (`KismetSystemLibrary.PrintString` (`KismetStringLibrary.Conv_DoubleToString` _output_get) true true (struct :`G` 0.66 :`B` 1.0 :`A` 1.0) 8.0))

(fn `UserConstructionScript`)