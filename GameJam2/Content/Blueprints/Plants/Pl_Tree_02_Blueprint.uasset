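; Fruit tree actor that grows apples and lets the Farmer player pick them.
; BeginPlay caches three child actor locations as spawn points, and Tick uses a six-second Delay to spawn fruit there up to MaxFruit.
; Overlap flags the player as near; Tick then attaches the first fruit to an empty-handed Farmer requesting pickup.
; The near flag clears only on pickup, as no end-overlap handler exists.
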(event `self.ReceiveBeginPlay`
  (set `self.SpawnPlaces` (`|MakeArray` (`SceneComponent.K2_GetComponentLocation` (`self.ChildActor`)) (`SceneComponent.K2_GetComponentLocation` (`self.ChildActor1`)) (`SceneComponent.K2_GetComponentLocation` (`self.ChildActor2`)))))

(event `self.ReceiveActorBeginOverlap`
  (params (OtherActor :type "Actor Object Reference"))
  (if (`self.ActorHasTag` OtherActor "Player")
    (cast `/Game/Blueprints/Farmer` OtherActor)
    (set `self.PlayerIsNear` true)))

(event `self.ReceiveTick`
  (params (DeltaSeconds :type "Float (single-precision)"))
  (bind _fuitsontree (`self.FuitsOnTree`))
  (bind _numberoffruit (`self.NumberOfFruit`))
  (bind _fuitsontree_2 (`self.FuitsOnTree`))
  (bind _output (`|GetArrayItem` _fuitsontree))
  (`|ExecutionSequence`
    (:`then_0`
      (if (< _numberoffruit (`self.MaxFruit`))
        (`KismetSystemLibrary.Delay` 6.0)
        (bind _returnvalue (`|SpawnActorFromClass` "/Game/Blueprints/Fruits_Veggies/FruitApple.FruitApple_C" (`KismetMathLibrary.Conv_VectorToTransform` (`|GetArrayItem` (`self.SpawnPlaces`) _numberoffruit)) "Undefined" "OverrideRootScale" null null))
        (`KismetArrayLibrary.Array_Add` _fuitsontree_2 _returnvalue)
        (`KismetArrayLibrary.Array_Set` _fuitsontree_2 _numberoffruit _returnvalue)
        (set `self.NumberOfFruit` (+ _numberoffruit 1))))
    (:`then_1`
      (bind _asfarmer (cast `/Game/Blueprints/Farmer` (stale `self.ReceiveActorBeginOverlap` OtherActor)))
      (if (> (`self.NumberOfFruit`) -1)
        (if (`self.PlayerIsNear`)
          (if (== (`/Game/Blueprints/Farmer.HoldingNumberOfItems` _asfarmer) 0)
            (if (`/Game/Blueprints/Farmer.PickUpAFruit` _asfarmer)
              (`self.K2_SetActorTransform` _output (`KismetMathLibrary.Conv_VectorToTransform` (-70.0 0.0 0.0)) false false)
              (`self.K2_AttachToActor` _output _asfarmer "None" "KeepRelative" "KeepRelative" "KeepRelative" true)
              (`KismetArrayLibrary.Array_RemoveItem` _fuitsontree _output)
              (set `self.NumberOfFruit` (- (`self.NumberOfFruit`) 1))
              (set `/Game/Blueprints/Farmer.HoldingNumberOfItems` 1 _asfarmer)
              (set `self.PlayerIsNear` false))))))))

(fn `UserConstructionScript`)