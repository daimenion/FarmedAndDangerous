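; BananaTree is a plant Blueprint for a banana tree that bears banana fruit and has a matching seed.
; On BeginPlay it sets the inherited fruit type, fruit limit, health, fruit timing and seed, then calls the parent BeginPlay.
; It is a data-only style child with no logic of its own, leaving plant behavior to the parent class.
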(event `self.ReceiveBeginPlay`
  (set `self.Fruits` "/Game/Blueprints/Fruits_Veggies/FruitBanana.FruitBanana_C")
  (set `self.MaxFruit` 2)
  (set `self.Health` 40.0)
  (set `self.FruitTime` 5.5)
  (set `self.Seed` "/Game/Blueprints/Plants/BananaSeed.BananaSeed_C")
  (`parent.ReceiveBeginPlay`))

(fn `UserConstructionScript`
  (`parent.UserConstructionScript`))