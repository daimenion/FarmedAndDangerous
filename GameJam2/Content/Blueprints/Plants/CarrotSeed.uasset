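; CarrotSeed is a plant seed Blueprint that configures the carrot version of a parent seed class.
; BeginPlay assigns the plant and CarrotTree types, growth timings and price before calling the parent logic.
; Tick runs the parent update, then casts MyTree to CarrotTree and destroys both the tree and the seed once it is picked.
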(event `self.ReceiveBeginPlay`
  (set `self.plant` "/Game/Blueprints/Plants/Pl_plant_03_Blueprint.Pl_plant_03_Blueprint_C")
  (set `self.Tree` "/Game/Blueprints/Plants/CarrotTree.CarrotTree_C")
  (set `self.PlantTime` 5.0)
  (set `self.TreeTime` 3.0)
  (set `self.Price` 4.0)
  (`parent.ReceiveBeginPlay`))

(event `self.ReceiveActorBeginOverlap`
  (params (OtherActor :type "Actor Object Reference"))
  (`parent.ReceiveActorBeginOverlap` OtherActor))

(event `self.ReceiveTick`
  (params (DeltaSeconds :type "Float (single-precision)"))
  (bind _mytree (`self.myTree`))
  (`parent.ReceiveTick` DeltaSeconds)
  (if (`KismetSystemLibrary.IsValid` _mytree)
    (bind _ascarrot_tree (cast `/Game/Blueprints/Plants/CarrotTree` _mytree))
    (if (`/Game/Blueprints/Plants/TreeParents.isPicked` _ascarrot_tree)
      (`self.K2_DestroyActor` _mytree)
      (`self.K2_DestroyActor`))))

(fn `UserConstructionScript`
  (`parent.UserConstructionScript`))