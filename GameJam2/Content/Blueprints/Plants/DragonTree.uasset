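; Dragon tree plant Blueprint, a data-only style child that configures a fruit-bearing plant growing dragon fruit.
; On BeginPlay it sets the fruit class, fruit cap, health, fruit timer and seed, then calls the parent BeginPlay, leaving plant behavior to the parent class.
; The grow speed multiplier assignment is unconnected and never runs, and the overlap and Tick events are disabled.
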(event `self.ReceiveBeginPlay`
  (set `self.Fruits` "/Game/Blueprints/Fruits_Veggies/FruitDragon.FruitDragon_C")
  (set `self.MaxFruit` 1)
  (set `self.Health` 30.0)
  (set `self.FruitTime` 7.0)
  (set `self.Seed` "/Game/Blueprints/Plants/DragonSeed.DragonSeed_C")
  (`parent.ReceiveBeginPlay`))

(fn `UserConstructionScript`
  (`parent.UserConstructionScript`))