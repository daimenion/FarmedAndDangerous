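; WatermelonTree is a plant Blueprint for a watermelon-bearing tree, configured as a child of a parent class.
; On BeginPlay it sets the fruit class, fruit limit, health, fruit timing and seed type, then calls the parent's BeginPlay.
; It adds no other logic: overlap and tick events are disabled, and the construction script only calls the parent.
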(event `self.ReceiveBeginPlay`
  (set `self.Fruits` "/Game/Blueprints/Fruits_Veggies/FruitWatermelon.FruitWatermelon_C")
  (set `self.MaxFruit` 1)
  (set `self.Health` 30.0)
  (set `self.FruitTime` 8.0)
  (set `self.Seed` "/Game/Blueprints/Plants/WatermelonSeed.WatermelonSeed_C")
  (`parent.ReceiveBeginPlay`))

(fn `UserConstructionScript`
  (`parent.UserConstructionScript`))