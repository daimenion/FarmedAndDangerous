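; Coconut tree plant that sets its fruit, seed, health and growth values on BeginPlay, then defers to its parent.
; While the player is near, a Delay in Tick gates a periodic random roll to drop the last coconut on the tree.
; A drop enables physics, detaches the coconut, updates the fruit list and count, flags it as falling and plays a fall sound event.
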(event `self.ReceiveBeginPlay`
  (set `self.Fruits` "/Game/Blueprints/Fruits_Veggies/FruitCoconut.FruitCoconut_C")
  (set `self.MaxFruit` 2)
  (set `self.Health` 40.0)
  (set `self.FruitTime` 7.0)
  (set `self.Seed` "/Game/Blueprints/Plants/CoconutSeed.CoconutSeed_C")
  (`parent.ReceiveBeginPlay`))

(event `self.ReceiveTick`
  (params (DeltaSeconds :type "Float (single-precision)"))
  (bind _fuitsontree (`self.FuitsOnTree`))
  (bind _output (`|GetArrayItem` _fuitsontree (- (`KismetArrayLibrary.Array_Length` (`self.FuitsOnTree`)) 1)))
  (`parent.ReceiveTick` DeltaSeconds)
  (if (`self.PlayerIsNear`)
    (`KismetSystemLibrary.Delay` 3.0)
    (if (>= (`KismetMathLibrary.RandomFloatInRange` 0.0 100.0) 75.0)
      (bind _asfruit_parent (cast `/Game/Blueprints/Fruits_Veggies/FruitParent` _output))
      (bind _asfruit_coconut (cast `/Game/Blueprints/Fruits_Veggies/FruitCoconut` _asfruit_parent))
      (`PrimitiveComponent.SetSimulatePhysics` (`/Game/Blueprints/Fruits_Veggies/FruitParent.Fruits` _asfruit_parent) true)
      (`self.K2_DetachFromActor` _output "KeepWorld" "KeepWorld" "KeepWorld")
      (`KismetArrayLibrary.Array_RemoveItem` _fuitsontree _output)
      (set `self.NumberOfFruit` (- (`self.NumberOfFruit`) 1))
      (set `/Game/Blueprints/Fruits_Veggies/FruitCoconut.Falling` true _asfruit_coconut)
      (`FMODBlueprintStatics.PlayEventAtLocation` "/Game/FMOD/Events/Other/CoconutFall.CoconutFall" (`self.GetTransform`)))))

(fn `UserConstructionScript`
  (`parent.UserConstructionScript`))