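; Base tree plant that grows fruit at three child-actor slots for its owning player's Farmer to pick and carry.
; BeginPlay line-traces for the Grid beneath it, whose growth and fertilizer states boost fruit timing and damage.
; Tick drives everything through Delays and polling: spawning fruit, handing it to a nearby empty-handed Farmer, fire damage and health bar updates.
; At zero health it spawns a destroyed Seed and removes itself and its fruit.
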(event `self.ReceiveActorEndOverlap`
  (params (OtherActor :type "Actor Object Reference")))

(event `self.ReceiveBeginPlay`
  (bind _returnvalue (`self.K2_GetActorLocation`))
  (if (`self.LoadOut`)
    (set `self.FruitTime` 0.0)
    (set `self.StartingFruitTime` 0.0))
  (set `self.SpawnPlaces` (`|MakeArray` (`SceneComponent.K2_GetComponentLocation` (`self.ChildActor`)) (`SceneComponent.K2_GetComponentLocation` (`self.ChildActor1`)) (`SceneComponent.K2_GetComponentLocation` (`self.ChildActor2`))))
  (bind _ashealth (cast `/Game/Blueprints/UI/Health` (`WidgetComponent.GetUserWidgetObject` (`self.HealthBar`))))
  (`KismetSystemLibrary.Delay` 0.05)
  (set `/Game/Blueprints/UI/Health.MaxHealth` (`self.Health`) _ashealth)
  (set `self.StartingFruitTime` (`self.FruitTime`))
  ;[1 1 1] Finding grid that tree is planted on
  (bind _outhit (`KismetSystemLibrary.LineTraceSingleForObjects` :`Start` (+ _returnvalue (0.0 50.0 200.0)) :`End` (+ _returnvalue (0.0 50.0 -200.0)) :`ObjectTypes` (`self.<WorldDynamic> Setter`) :`TraceColor` (struct :`G` 0.088855 :`B` 1.0 :`A` 1.0)))
  (set `self.Nearest Grid` (`.HitActor` (`GameplayStatics.BreakHitResult` _outhit))))

(event `self.Capsule.OnComponentEndOverlap`
  (params (OverlappedComponent :type "PrimitiveComponent Object Reference") (OtherActor :type "Actor Object Reference") (OtherComp :type "PrimitiveComponent Object Reference") (OtherBodyIndex :type Integer))
  (if (`self.ActorHasTag` OtherActor "Player")
    (set `self.PlayerIsNear` false)))

(event `self.ReceiveActorBeginOverlap`
  (params (OtherActor :type "Actor Object Reference")))

(event `self.Capsule.OnComponentBeginOverlap`
  (params (OverlappedComponent :type "PrimitiveComponent Object Reference") (OtherActor :type "Actor Object Reference") (OtherComp :type "PrimitiveComponent Object Reference") (OtherBodyIndex :type Integer) (bFromSweep :type Boolean) (SweepResult :type "HitResult Structure (by ref)"))
  (if (`self.ActorHasTag` OtherActor "Player")
    (set `self.PlayerIsNear` true)))

(event `self.ReceiveTick`
  (params (DeltaSeconds :type "Float (single-precision)"))
  (bind _returnvalue (`self.GetTransform`))
  (bind _fuitsontree (`self.FuitsOnTree`))
  (bind _fuitsontree_2 (`self.FuitsOnTree`))
  (bind _numberoffruit (`self.NumberOfFruit`))
  (bind _fuitsontree_3 (`self.FuitsOnTree`))
  (bind _health (`self.Health`))
  (bind _nearest_grid (`self.Nearest Grid`))
  (bind _originaldamage (`self.originalDamage`))
  (bind _array (`|MakeArray` (`self.ChildActor`) (`self.ChildActor1`) (`self.ChildActor2`)))
  (bind _output (`|GetArrayItem` _array _numberoffruit))
  (bind _output_2 (`|GetArrayItem` _fuitsontree_2 (- (`KismetArrayLibrary.Array_Length` _fuitsontree_2) 1)))
  (`|ExecutionSequence`
    (:`then_0`
      (if (< _numberoffruit (`self.MaxFruit`))
        (`KismetSystemLibrary.Delay` (`self.FruitTime`))
        (set `self.Waiting` false)
        (if (== (`KismetArrayLibrary.Array_Length` (`SceneComponent.GetChildrenComponents` _output false)) 0)
          (bind _returnvalue_2 (`|SpawnActorFromClass` (`self.Fruits`) (`KismetMathLibrary.Conv_VectorToTransform` (`|GetArrayItem` (`self.SpawnPlaces`) _numberoffruit)) "Undefined" "OverrideRootScale" null null))
          (bind _returnvalue_3 (`KismetArrayLibrary.Array_Add` _fuitsontree _returnvalue_2))
          (if (== (stale _array_index) 1)
            (`KismetArrayLibrary.Array_Set` _fuitsontree_3 2 (stale _returnvalue_4))
            (else
              (`KismetArrayLibrary.Array_Set` _fuitsontree _returnvalue_3 _returnvalue_2)))
          (`self.K2_AttachToComponent` _returnvalue_2 _output "None" "KeepWorld" "KeepWorld" "KeepWorld" true)
          (set `self.NumberOfFruit` (+ _numberoffruit 1))
          (bind _asfruit_parent (cast `/Game/Blueprints/Fruits_Veggies/FruitParent` _returnvalue_2))
          (set `/Game/Blueprints/Fruits_Veggies/FruitParent.OwningPlayer` (`self.OwningPlayer`) _asfruit_parent)
          (set `self.originalDamage` (`/Game/Blueprints/Fruits_Veggies/FruitParent.damage` _asfruit_parent))
          (else
            (for (_array_element _array_index) _array
              (if (== (`KismetArrayLibrary.Array_Length` (`SceneComponent.GetChildrenComponents` _array_element false)) 0)
                (bind _returnvalue_4 (`|SpawnActorFromClass` (`self.Fruits`) (`KismetMathLibrary.Conv_VectorToTransform` (`|GetArrayItem` (`self.SpawnPlaces`) _array_index)) "Undefined" "OverrideRootScale" null null))
                (bind _returnvalue_5 (`KismetArrayLibrary.Array_Add` _fuitsontree_3 _returnvalue_4))
                (`KismetArrayLibrary.Array_Set` _fuitsontree_3 _returnvalue_5 _returnvalue_4)
                (`self.K2_AttachToComponent` _returnvalue_4 _array_element "None" "KeepWorld" "KeepWorld" "KeepWorld" true)
                (set `self.NumberOfFruit` (+ _numberoffruit 1))
                (bind _asfruit_parent_2 (cast `/Game/Blueprints/Fruits_Veggies/FruitParent` _returnvalue_4))
                (set `/Game/Blueprints/Fruits_Veggies/FruitParent.OwningPlayer` (`self.OwningPlayer`) _asfruit_parent_2)
                (set `self.originalDamage` (`/Game/Blueprints/Fruits_Veggies/FruitParent.damage` _asfruit_parent_2))))))))
    (:`then_1`
      ;[1 1 1] Sprinkler Stuff
      (bind _asgrid (cast `/Game/Blueprints/Grid/Grid` _nearest_grid))
      (if (`/Game/Blueprints/Grid/Grid.GrowMultiplier` _asgrid)
        (if (`self.tempLocker`)
          (set `self.tempLocker` false)
          (set `self.FruitTime` (/ (`self.FruitTime`) (`self.growSpeedMultiplier`))))
        (else
          (set `self.FruitTime` (`self.StartingFruitTime`))
          (set `self.tempLocker` true))))
    (:`then_2`
      (if (`self.OnFire`)
        (`|ExecutionSequence`
          (:`then_0`
            (`KismetSystemLibrary.Delay` 1.0)
            (set `self.Health` (- (`self.Health`) (`self.BurnDMG`))))
          (:`then_1`
            (`KismetSystemLibrary.Delay` 10.0)
            (set `self.OnFire` false)))
        (else
          (bind _outactors (`GameplayStatics.GetAllActorsOfClass` "/Game/Blueprints/Farmer.Farmer_C"))
          (for _array_element_2 _outactors
            (bind _asfarmer (cast `/Game/Blueprints/Farmer` _array_element_2))
            (if (== (`/Game/Blueprints/Farmer.HoldingNumberOfItems` _asfarmer) 0)
              (if (and (`self.IsOverlappingActor` _array_element_2 self) (== (`/Game/Blueprints/Farmer.PlayerNumber` _asfarmer) (`self.OwningPlayer`)))
                (if (> (`self.NumberOfFruit`) 0)
                  (if (`self.PlayerIsNear`)
                    (if (`/Game/Blueprints/Farmer.PickUpAFruit` _asfarmer)
                      (`self.K2_SetActorTransform` _output_2 (`KismetMathLibrary.Conv_VectorToTransform` (70.0 0.0 -20.0)) false false)
                      (`self.K2_DetachFromActor` _output_2 "KeepWorld" "KeepWorld" "KeepWorld")
                      (`self.K2_AttachToActor` _output_2 _asfarmer "None" "KeepRelative" "KeepRelative" "KeepRelative" true)
                      (`KismetArrayLibrary.Array_RemoveItem` _fuitsontree_2 _output_2)
                      (set `self.NumberOfFruit` (- (`self.NumberOfFruit`) 1))
                      (set `/Game/Blueprints/Farmer.HoldingNumberOfItems` 1 _asfarmer)
                      (set `self.isPicked` true)
                      (if (`self.ActorHasTag` "Ground")
                        (set `/Game/Blueprints/Farmer.Ground` true _asfarmer)
                        (elif (`self.ActorHasTag` "Heavy")
                          (set `/Game/Blueprints/Farmer.Heavy` true _asfarmer)
                          (else
                            (set `/Game/Blueprints/Farmer.High` true _asfarmer)))))))))))))
    (:`then_3`
      (bind _ashealth (cast `/Game/Blueprints/UI/Health` (`WidgetComponent.GetUserWidgetObject` (`self.HealthBar`))))
      (set `/Game/Blueprints/UI/Health.CurrentHealth` _health _ashealth)
      (if (<= _health 0.0)
        (`FMODBlueprintStatics.PlayEventAtLocation` "/Game/FMOD/Events/ImpactSound/PlantImpact.PlantImpact" (`self.GetTransform`))
        (if true
          (bind _returnvalue_6 (`|SpawnActorFromClass` (`self.Seed`) (`KismetMathLibrary.MakeTransform` (`KismetMathLibrary.MakeVector` (- (.x (.location _returnvalue)) 125.0) (.y (.location _returnvalue)) (.z (.location _returnvalue))) (.rotation _returnvalue) (.scale _returnvalue)) "Undefined" "OverrideRootScale" null null))
          (bind _asseed (cast `/Game/Blueprints/Plants/Seed` _returnvalue_6))
          (set `/Game/Blueprints/Plants/Seed.destroyed` true _asseed)
          (`self.K2_DestroyActor`)
          (for _array_element_3 (`self.FuitsOnTree`)
            (`self.K2_DestroyActor` _array_element_3)))))
    (:`then_4`
      (bind _asgrid_2 (cast `/Game/Blueprints/Grid/Grid` _nearest_grid))
      (for _array_element_4 (`self.FuitsOnTree`)
        (bind _asfruit_parent_3 (cast `/Game/Blueprints/Fruits_Veggies/FruitParent` _array_element_4))
        (if (`/Game/Blueprints/Grid/Grid.Fertilized` _asgrid_2)
          (set `/Game/Blueprints/Fruits_Veggies/FruitParent.damage` (* _originaldamage (`self.damageMultiplier`)) _asfruit_parent_3)
          (else
            (set `/Game/Blueprints/Fruits_Veggies/FruitParent.damage` _originaldamage _asfruit_parent_3)))))))

(fn `Timer`
  (params (NewParam1 :type "Float (double-precision)"))
  (returns (done :type Boolean))
  (bind _result (`/Engine/EditorBlueprintResources/StandardMacros.IncrementFloat` (`self.Time`))
    (:`  `
      (if (>= _result (* NewParam1 1000.0))
        (set `self.Time` 0.0)
        (return true)))))

(fn `UserConstructionScript`)