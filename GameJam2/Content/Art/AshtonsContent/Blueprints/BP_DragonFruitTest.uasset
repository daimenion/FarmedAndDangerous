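; BP_DragonFruitTest is a test effect actor that plays a dragon fruit flame particle effect with a burned-ground decal, then destroys itself.
; The construction script creates a dynamic burn material, and BeginPlay activates the particle component, whose activation event shows the decal and starts a timeline.
; The timeline drives flame size and ground burn, shuts off the particles through an event track, and destroys the actor shortly after finishing.
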(event `self.ReceiveBeginPlay`
  (`ActorComponent.Activate` (`self.DragonFruit`) false))

(event `self.DragonFruit.OnComponentActivated`
  (params (Component :type "ActorComponent Object Reference") (bReset :type Boolean))
  (bind _burnedspot (`self.BurnedSpot`))
  (`SceneComponent.SetVisibility` _burnedspot true false)
  (`DecalComponent.SetDecalMaterial` _burnedspot (`self.DynamicMaterial`))
  (bind (_direction _groundburn _flamesize) (`Timeline|Timeline_0` :!via `PlayFromStart`)
    (:`Update`
      (`FXSystemComponent.SetVectorParameter` (`self.DragonFruit`) "FlameSize" _flamesize)
      (`MaterialInstanceDynamic.SetScalarParameterValue` (`self.DynamicMaterial`) "GroundBurn" _groundburn))
    (:`Finished`
      (`KismetSystemLibrary.Delay` 3.0)
      (`self.K2_DestroyActor`))
    (:`Deactivate`
      (`ActorComponent.Deactivate` (`self.DragonFruit`)))))

(fn `UserConstructionScript`
  (bind _returnvalue (`KismetMaterialLibrary.CreateDynamicMaterialInstance` "/Game/Art/AshtonsContent/Materials/Instanced/INT_BurnedGround.INT_BurnedGround" "DM_Burn"))
  (set `self.DynamicMaterial` _returnvalue))