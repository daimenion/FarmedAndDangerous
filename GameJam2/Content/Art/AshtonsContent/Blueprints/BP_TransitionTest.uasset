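; BP_TransitionTest is a test actor that burns an apple tree mesh away to ash, then destroys itself.
; BeginPlay staggers the fire particles and starts looping ash; the last fire's activation plays a timeline driving the material's Burn and FadeAway parameters for a masked burnt blend.
; Delays chained from the timeline update swap the looping effects for ash bursts, hide the mesh, disable its collision and finally destroy the actor.
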(event `self.ReceiveBeginPlay`
  ;[1 1 1] Activate 3 particles, delay to give a "grow" with the flames
  (`ActorComponent.Activate` (`self.Fire1`) false)
  (`ActorComponent.Activate` (`self.Fire2`) false)
  (`ActorComponent.Activate` (`self.pp_AshDebrieLoop`) false)
  (`KismetSystemLibrary.Delay` 1.0)
  (`ActorComponent.Activate` (`self.Fire3`) false))

(event `self.Fire3.OnComponentActivated`
  (params (Component :type "ActorComponent Object Reference") (bReset :type Boolean))
  (bind _mainmesh (`self.MainMesh`))
  (bind _mainmesh_2 (`self.MainMesh`))
  ;[1 1 1] Once last fire has been activated a timeline of 3 seconds will lerp into a burnt blend from material using a mask
  (bind (_direction _burnvalue _fadeaway) (`Timeline|BurnTimeline`)
    (:`Update`
      (`MeshComponent.SetScalarParameterValueOnMaterials` _mainmesh "Burn" _burnvalue)
      (`MeshComponent.SetScalarParameterValueOnMaterials` _mainmesh "FadeAway" _fadeaway)
      ;[1 1 1] After 10 seconds the looping fire and ashes will deactivate, then burst Ash will activate
      (`KismetSystemLibrary.Delay` 7.0)
      (`ActorComponent.Deactivate` (`self.Fire1`))
      (`ActorComponent.Deactivate` (`self.Fire3`))
      (`ActorComponent.Deactivate` (`self.Fire2`))
      (`ActorComponent.Deactivate` (`self.pp_AshDebrieLoop`))
      (`ActorComponent.Activate` (`self.pp_AshDebrie`) false)
      (`ActorComponent.Activate` (`self.pp_AshDebrie1`) false)
      ;[1 1 1] Delay for to set visibility of apple tree, and collision off, last delay is so can see the effects of the ashes fly in the sky
      (`KismetSystemLibrary.Delay` 2.0)
      (`SceneComponent.SetVisibility` _mainmesh_2 false false)
      (`PrimitiveComponent.SetCollisionEnabled` _mainmesh_2 "NoCollision")
      (`KismetSystemLibrary.Delay` 8.0)
      (`self.K2_DestroyActor`))))

(fn `UserConstructionScript`)