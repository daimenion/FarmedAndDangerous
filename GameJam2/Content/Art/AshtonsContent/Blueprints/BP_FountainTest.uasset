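; BP_FountainTest is a fountain test actor that spins its mesh and leaves splat decals where its particles land.
; Each tick, RotatingMesh gets a small fixed yaw increment that is not scaled by delta time.
; When ParticleSystem reports a particle collision, it spawns a random SplatDecals material at the hit location, oriented along the collision direction, which fades out over a few seconds.
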(event `self.ReceiveTick`
  (params (DeltaSeconds :type "Float (single-precision)"))
  ;[1 1 1] Rotates the Mesh/Particle Effect
  (`SceneComponent.K2_AddRelativeRotation` (`self.RotatingMesh`) (struct :`Yaw` 0.5) false false))

(event `self.ParticleSystem.OnParticleCollide`
  (params (EventName :type Name) (EmitterTime :type "Float (single-precision)") (ParticleTime :type Integer) (Location :type "Vector Structure") (Velocity :type "Vector Structure") (Direction :type "Vector Structure") (Normal :type "Vector Structure") (BoneName :type Name) (PhysMat :type "PhysicalMaterial Object Reference"))
  (bind _splatdecals (`self.SplatDecals`))
  ;[1 1 1] Adds decal from position where particles land in the world
  (bind _returnvalue (`GameplayStatics.SpawnDecalAtLocation` (`|GetArrayItem` _splatdecals (`KismetMathLibrary.RandomIntegerInRange` 0 (- (`KismetArrayLibrary.Array_Length` _splatdecals) 1))) (32.0 32.0 32.0) Location (`KismetMathLibrary.Conv_VectorToRotator` Direction) 8.0))
  (`DecalComponent.SetFadeOut` _returnvalue 0.0 6.5 true))

(fn `UserConstructionScript`)